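; Camera plane actor that sets up a material instance and syncs its transform from clients through the server.
; After a half-second delay, BeginPlay runs InitializeCameraPlane, stores the returned material and sets Pause, which despite its name enables the Tick logic.
; Each tick feeds the material to GlobalTick, and non-server instances send their transform by RPC into PawnTransform, whose OnRep moves the actor.
; The material instance's OnRep is empty.
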(event Custom|RPC%20Server%20Pawn%20Transform%20Replicate
  (params (transfirm :type Transform))
  (Variables|Default|SetpawnTransform transfirm))

(event EventBeginPlay
  (Utilities|FlowControl|Delay 0.5)
  (|CallParentFunction)
  (bind _thematerialinstance (CallFunction|InitializeCameraPlane))
  (Variables|Default|SetmyMaterialInstance _thematerialinstance)
  (Variables|Default|SetPause true))

(event EventTick
  (params (DeltaSeconds :type Float%20%28single-precision%29))
  (|CallParentFunction DeltaSeconds)
  (if (Variables|Default|GetPause)
    (CallFunction|GlobalTick (Variables|Default|GetmyMaterialInstance))
    (if (not (Networking|IsServer))
      (CallFunction|RPCServerPawnTransformReplicate (Transformation|GetActorTransform)))))

(fn ConstructionScript
  (|CallParentFunction))

(fn OnRepPawnTransform
  (Transformation|SetActorTransform (Variables|Default|GetpawnTransform)))

(fn OnRepMyMaterialInstance)