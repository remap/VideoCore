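; Video plane subclass that plays a recorded media source on the base plane's material, with toggleable playback, optional autoplay and looping.
; On BeginPlay it links media player, texture and sound, then opens the source URL, logging failures.
; Tick sets aspect ratio from video dimensions while the player is ready but not playing.
; It serializes as plane type 2, appending playback flags and file path to the parent's byte data.
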(event EventBeginPlay
  ;[0.02946 0.7995 1] begin
  (|CallParentFunction)
  (CallFunction|InitializeRecordedPlane)
  (if (.isRear (CallFunction|IsRearPlane self))
    (Variables|Default|SetautorotateLocalRotation "0,180.000000, 0")))

(event Collision|EventActorBeginOverlap
  (params (OtherActor :type Actor%20Object%20Reference)))

(event EventTick
  (params (DeltaSeconds :type Float%20%28single-precision%29))
  (bind _mediaplayer (Variables|Default|GetmediaPlayer))
  (bind _mediaplayer_2 (Variables|Default|GetmediaPlayer))
  (bind _returnvalue (Class|MediaPlayer|GetVideoTrackDimensions _mediaplayer_2))
  (bind (_x _y) (Utilities|Struct|BreakIntPoint _returnvalue))
  ;[1 0.1813 0.1116] tick
  (Utilities|FlowControl|Sequence
    (:then_0
      (CallFunction|PlaneBaseTick))
    (:then_1
      ;;[1 1 1] handle aspect ratio when media player is ready
      (Utilities|IsValid _mediaplayer
        (:Is%20Valid
          (if (Class|MediaPlayer|IsReady _mediaplayer)
            (if (not (Audio|Components|Audio|IsPlaying _mediaplayer))
              (CallFunction|SetAspectRatio (Math|Conversions|ToFloat(Integer) _x) (Math|Conversions|ToFloat(Integer) _y)))))))))

(fn ConstructionScript
  (|CallParentFunction))

(fn InitializeRecordedPlane
  (bind _mediatexture (Variables|Default|GetmediaTexture))
  (bind _mediaplayer (Variables|Default|GetmediaPlayer))
  (bind _mediasource (Variables|Default|GetmediaSource))
  (bind _mediaplayer_2 (Variables|Default|GetmediaPlayer))
  (bind _returnvalue (Class|MediaPlayer|GetUrl _mediaplayer_2))
  (bind _returnvalue_2 (Class|MediaSource|GetUrl _mediasource))
  (bind _returnvalue_3 (Utilities|Text|ToText(String) _returnvalue))
  (Utilities|FlowControl|Sequence
    (:then_0
      ;[1 1 1] setup material instance and media texture nad media sound
      (Utilities|IsValid _mediatexture
        (:Is%20Valid
          (Rendering|Material|SetTextureParameterValue (Variables|Default|GetmyMaterialInstance) "Texture" _mediatexture)
          (Media|MediaSoundComponent|SetMediaPlayer (Variables|Default|GetmediaTexture) (Variables|Default|GetmediaPlayer))
          (Media|MediaSoundComponent|SetMediaPlayer (Variables|Default|GetMediaSound) (Variables|Default|GetmediaPlayer))
          (if (Variables|Default|GetflipHorizontalOnConstruct)
            (CallFunction|FlipTextureHorizontal)))
        (:Is%20Not%20Valid
          (Class|DDBlueprintLibrary|LogError "Recorded plane: Media Texture is not set"))))
    (:then_1
      ;[1 1 1] media player setup
      (Utilities|IsValid _mediaplayer
        (:Is%20Valid
          (Variables|/Script/MediaAssets.MediaPlayer|SetPlayOnOpen _mediaplayer (Variables|Default|GetisAutoPlay))
          (Components|Timeline|SetLooping _mediaplayer (Variables|Default|GetisLooping))
          (Media|MediaPlayer|BindEventtoOnMediaOpened _mediaplayer_2 (EventDispatchers|CreateEvent :!event OnMediaOpenSucceded))
          (Media|MediaPlayer|BindEventtoOnMediaOpenFailed _mediaplayer_2 (EventDispatchers|CreateEvent :!event OnMediaOpenFailed))
          (Class|DDBlueprintLibrary|LogDebug (Utilities|String|ToString(Text) (Utilities|Text|FormatText "OPEN URL {url}" _returnvalue_3)))
          (Utilities|IsValid _mediasource
            (:Is%20Valid
              (Class|DDBlueprintLibrary|LogDebug (Utilities|String|ToString(Text) (Utilities|Text|FormatText "MEDIA SOURCE URL {url}" (Utilities|Text|ToText(String) _returnvalue_2))))
              (bind _returnvalue_4 (Class|MediaPlayer|OpenUrl (Variables|Default|GetmediaPlayer) _returnvalue_2))
              (if _returnvalue_4
                (Class|DDBlueprintLibrary|LogDebug (Utilities|String|ToString(Text) (Utilities|Text|FormatText "OPEN SUCCESS {url}" _returnvalue_3)))
                (else
                  (Class|DDBlueprintLibrary|LogError (Utilities|String|ToString(Text) (Utilities|Text|FormatText "OPEN FAILED {url}" _returnvalue_3))))))
            (:Is%20Not%20Valid
              (Class|DDBlueprintLibrary|LogError "MEDIA SOURCE IS NOT VALID WHY???"))))
        (:Is%20Not%20Valid
          (Class|DDBlueprintLibrary|LogError "Recorded plane: Media Player is not set"))))))

(fn GetMediaPlayer
  (return (Variables|Default|GetmediaPlayer)))

(fn GetMediaTexture
  (return (Variables|Default|GetmediaTexture)))

(fn SetMediaTexture
  (params (mediaTexture :type Media%20Texture%20Object%20Reference))
  (bind _output_get (Variables|Default|SetmediaTexture mediaTexture))
  (Media|MediaSoundComponent|SetMediaPlayer _output_get (Variables|Default|GetmediaPlayer)))

(fn DebugPlayerStateString
  (bind _mediaplayer (Variables|Default|GetmediaPlayer))
  (return (Utilities|Text|FormatText "buffering {b} closed {c} connecting {cn} looping {l} paused {p} playing {pp} preparing {pr} ready {r}" (Utilities|Text|ToText(Boolean) (Class|MediaPlayer|IsBuffering _mediaplayer)) (Utilities|Text|ToText(Boolean) (Class|MediaPlayer|IsClosed _mediaplayer)) (Utilities|Text|ToText(Boolean) (Class|MediaPlayer|IsConnecting _mediaplayer)) (Utilities|Text|ToText(Boolean) (Class|MediaPlayer|IsLooping _mediaplayer)) (Utilities|Text|ToText(Boolean) (Class|MediaPlayer|IsPaused _mediaplayer)) (Utilities|Text|ToText(Boolean) (Audio|Components|Audio|IsPlaying _mediaplayer)) (Utilities|Text|ToText(Boolean) (Class|MediaPlayer|IsPreparing _mediaplayer)) (Utilities|Text|ToText(Boolean) (Class|MediaPlayer|IsReady _mediaplayer)))))

(fn OnMediaOpenFailed
  (params (failedUrl :type String))
  (Class|DDBlueprintLibrary|LogError (Utilities|String|ToString(Text) (Utilities|Text|FormatText "Failed to open media at URL {url}" (Utilities|Text|ToText(String) failedUrl))))
  (CallFunction|DebugCheckMediaPlayerErrors))

(fn OnMediaOpenSucceded
  (params (openedUrl :type String))
  (Class|DDBlueprintLibrary|LogDebug (Utilities|String|ToString(Text) (Utilities|Text|FormatText "Media opened successfully: {url}" (Utilities|Text|ToText(String) openedUrl))))
  (CallFunction|DebugCheckMediaPlayerErrors))

(fn DebugCheckMediaPlayerErrors
  (if (Media|MediaPlayer|HasError (Variables|Default|GetmediaPlayer))
    (Class|DDBlueprintLibrary|LogError "Media player has errors")
    (Class|DDBlueprintLibrary|LogError (Utilities|String|ToString(Text) (CallFunction|DebugPlayerStateString)))))

(fn TogglePlayback
  (bind _mediaplayer (Variables|Default|GetmediaPlayer))
  (if (Audio|Components|Audio|IsPlaying _mediaplayer)
    (Sequencer|Player|Pause _mediaplayer)
    (else
      (Media|MediaPlayer|Play _mediaplayer :!class /Script/MediaAssets.MediaPlayer))))

(fn SerializePlaneData
  (bind _mediasource (Variables|Default|GetmediaSource))
  (bind _filepath (Variables|/Script/MediaAssets.FileMediaSource|GetFilePath _mediasource))
  (bind _returnvalue (Utilities|String|Len _filepath))
  (bind _returnvalue_2 (Math|Conversions|ToByte(Integer) _returnvalue))
  (bind _data (|CallParentFunction))
  ;[1 1 1] type 2 - recorded planes
  (Utilities|Array|Add _data 2)
  (Utilities|Array|Add _data (Math|Conversions|ToByte(Integer) (Variables|Default|GetisAutoPlay)))
  (Utilities|Array|Add _data (Math|Conversions|ToByte(Integer) (Variables|Default|GetisLooping)))
  (Utilities|Array|Add _data _returnvalue_2)
  (bind _returnvalue_3 (Class|VideoCoreFunctionLibrary|StringtoByteArray (Utilities|String|GetSubstring _filepath 0 (Math|Conversions|ToInteger(Byte) _returnvalue_2))))
  (Utilities|Array|AppendArray _data _returnvalue_3)
  (return _data))

(fn InitfromSerializedData0
  (params (data :type Array%20of%20Bytes))
  (bind _output (Utilities|Array|Get(acopy) data))
  (if (== _output 2)
    (Utilities|Array|RemoveIndex data)
    (Variables|Default|SetisAutoPlay (== (Utilities|Array|Get(acopy) data) 1))
    (Utilities|Array|RemoveIndex data)
    (Variables|Default|SetisLooping (== (Utilities|Array|Get(acopy) data) 1))
    (Utilities|Array|RemoveIndex data)
    (bind _returnvalue (Class|VideoCoreFunctionLibrary|ByteArraytoString (CallFunction|SliceArray data 1 (Math|Conversions|ToInteger(Byte) (Utilities|Array|Get(acopy) data)))))
    (Class|FileMediaSource|SetFilePath (Variables|Default|GetmediaSource) _returnvalue)
    (return false)
    (else
      (Class|DDBlueprintLibrary|LogWarning (Utilities|String|ToString(Text) (Utilities|Text|FormatText "Can't initialize Recorded plane. Plane type is {t}" _output)))
      (return false))))

(fn FlipTextureHorizontal
  (bind _mymaterialinstance (Variables|Default|GetmyMaterialInstance))
  (bind _isa (Utilities|FlowControl|FlipFlop)
    (:A
      _)
    (:B
      _))
  (Rendering|Material|SetScalarParameterValue _mymaterialinstance "u1" (Math|Float|SelectFloat 1.0 0.0 _isa) :!class /Script/Engine.MaterialInstanceDynamic)
  (Rendering|Material|SetScalarParameterValue _mymaterialinstance "u2" (- 1.0 (Math|Float|SelectFloat 1.0 0.0 _isa)) :!class /Script/Engine.MaterialInstanceDynamic))

(fn PostDeserializeInit
  (bind _mediaplayer (Variables|Default|GetmediaPlayer))
  (|CallParentFunction)
  (Variables|/Script/MediaAssets.MediaPlayer|SetPlayOnOpen _mediaplayer (Variables|Default|GetisAutoPlay))
  (Components|Timeline|SetLooping _mediaplayer (Variables|Default|GetisLooping)))