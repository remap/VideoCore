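; Actor component that streams audio/video between multiplayer clients over VideoCore RTC, using a media sender and receiver it creates.
; Role follows the top owner: local PlayerController sends from a render target, others receive.
; With sync on, server RPCs multicast produce start/stop to drive consumption; with it off, senders can also consume and consuming is triggered separately.
; Mirrored track states and stream hints let receivers catch up when signaling initializes.
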(event Custom|Setup%20Media%20Sender%20Callbacks
  (bind _mediasender (Variables|Default|GetmediaSender))
  ;[1 0.06771 0.06771] VideoCoreMediaSender Callbacks
  (EventDispatchers|BindEventtoOnStartProducing _mediasender (delegate Custom|On%20Start%20Producing%20Stream))
  (EventDispatchers|BindEventtoOnProduceFailure _mediasender (delegate Custom|On%20Produce%20Failure))
  (EventDispatchers|BindEventtoOnStoppedProducing _mediasender (delegate Custom|On%20Stopped%20Producing%20Stream)))

(event Custom|On%20Start%20Producing%20Stream
  (params (StreamId :type String) (Kind :type EMediaTrackKind%20Enum :default "Unknown"))
  ;[1 0.06771 0.06771] VideoCoreMediaSender Callbacks
  (Utilities|SenderUpdateTrackState Kind)
  (Utilities|SwitchonSendRecvSync
    (:Sync%20ON
      (CallFunction|ServerSenderStartedStreamProduce "" StreamId (CallFunction|GetStreamHint Kind) Kind)
      (Class|DDBlueprintLibrary|LogWarning "NDI-RTC plane: started producing"))))

(event Custom|On%20Streaming%20Started
  (params (ProducerId :type String) (Kind :type EMediaTrackKind%20Enum :default "Unknown"))
  ;[0 0.978 1] VideoCoreMediaReceiver Callbacks
  (Class|DDBlueprintLibrary|LogTrace (Utilities|String|ToString(Text) (Utilities|Text|FormatText "Started consuming from {id}" ProducerId))))

(event Custom|Server%20Sender%20Stopped%20Stream%20Produce
  (params (streamId :type String) (streamHint :type String) (kind :type EMediaTrackKind%20Enum :default "Unknown"))
  ;[1 1 1] mplayer handling
  ;;[0.7917 0.0378 0.2869] stop produce - stop consume (sync ON only)
  (CallFunction|MCastSenderStoppedStreamProduce streamId streamHint kind))

(event Custom|Server%20Sender%20Started%20Stream%20Produce
  (params (clientId :type String) (streamId :type String) (streamHint :type String) (kind :type EMediaTrackKind%20Enum :default "Unknown"))
  ;[1 1 1] mplayer handling
  ;;[0 0.7035 1] start produce -> start consume (sync ON only)
  (CallFunction|McastSenderStartedStreamProduce clientId streamId streamHint kind))

(event Custom|MCast%20Sender%20Stopped%20Stream%20Produce
  (params (streamId :type String) (streamHint :type String) (kind :type EMediaTrackKind%20Enum :default "Unknown"))
  ;[1 1 1] mplayer handling
  ;;[0.7917 0.0378 0.2869] stop produce - stop consume (sync ON only)
  (CallFunction|StopConsume))

(event Custom|Server%20Set%20Sync
  (params (syncValue :type Boolean))
  ;[1 1 1] mplayer handling
  (Variables|Default|SetsyncSenderReceiver syncValue))

(event Custom|Server%20Start%20Consume
  ;[1 1 1] mplayer handling
  ;;[1 0.1747 0.2345] start consume (sync OFF only)
  (CallFunction|McastStartConsume))

(event Custom|Mcast%20Start%20Consume
  ;[1 1 1] mplayer handling
  ;;[1 0.1747 0.2345] start consume (sync OFF only)
  (Utilities|SwitchonSendRecvSync
    (:Sync%20OFF
      (CallFunction|StartConsume "" "Video"))))

(event Custom|Setup%20Signaling%20Callbacks
  (params (rtcSignaling :type Video%20Core%20Signaling%20Component%20Object%20Reference))
  ;[1 0.8671 0] handle case when signaling has not initialized yet
  (EventDispatchers|BindEventtoOnRtcSubsystemInitialized rtcSignaling (delegate Custom|On%20Signaling%20Initialized)))

(event Custom|Server%20Set%20Stream%20Hint
  (params (hint :type String) (kind :type EMediaTrackKind%20Enum :default "Unknown"))
  ;[1 1 1] mplayer handling
  (CallFunction|SetStreamHint hint kind))

(event Custom|On%20Signaling%20Initialized
  (params (MyCaps :type SIO%20Json%20Object%20Object%20Reference))
  ;[1 0.8671 0] handle case when signaling has not initialized yet
  (Utilities|SwitchbyRole
    (:Sender
      (CallFunction|UpdateClientId))
    (:Receiver
      (CallFunction|ValidateStreamState "Audio" :!label _label)
      (CallFunction|ValidateStreamState "Video"))
    (:Unowned
      (goto _label))))

(event Custom|On%20Produce%20Failure
  (params (StreamId :type String) (Kind :type EMediaTrackKind%20Enum :default "Unknown") (Reason :type String))
  ;[1 0.06771 0.06771] VideoCoreMediaSender Callbacks
  (Utilities|SenderUpdateTrackState Kind)
  (Utilities|SwitchonSendRecvSync
    (:Sync%20ON
      (CallFunction|ServerSenderStoppedStreamProduce StreamId (CallFunction|GetStreamHint Kind) Kind)
      (Class|DDBlueprintLibrary|LogWarning (Utilities|String|ToString(Text) (Utilities|Text|FormatText "NDI-RTC plane: produce failed: {m}" Reason))))))

(event Custom|Server%20Set%20Track%20State
  (params (kind :type EMediaTrackKind%20Enum :default "Unknown") (state :type EMediaTrackState%20Enum :default "Unknown"))
  ;[1 1 1] mplayer handling
  (CallFunction|UpdateTrackState kind state))

(event Custom|On%20Stopped%20Producing%20Stream
  (params (StreamId :type String) (Kind :type EMediaTrackKind%20Enum :default "Unknown") (Reason :type String))
  ;[1 0.06771 0.06771] VideoCoreMediaSender Callbacks
  (Utilities|SenderUpdateTrackState Kind)
  (Utilities|SwitchonSendRecvSync
    (:Sync%20ON
      (CallFunction|ServerSenderStoppedStreamProduce StreamId (CallFunction|GetStreamHint Kind) Kind)
      (Class|DDBlueprintLibrary|LogWarning (Utilities|String|ToString(Text) (Utilities|Text|FormatText "NDI-RTC plane: produce stopped: {m}" Reason))))))

(event Custom|Server%20Set%20Sender%20Client%20Id
  (params (clientId :type String))
  ;[1 1 1] mplayer handling
  (Variables|Default|SetsenderClientId clientId))

(event Custom|On%20Client%20State%20Changed
  (params (State :type EClientState%20Enum :default "Offline"))
  ;[0 0.978 1] VideoCoreMediaReceiver Callbacks
  (Class|DDBlueprintLibrary|LogTrace (Utilities|String|ToString(Text) (Utilities|Text|FormatText "Client state changed: {st}" (Utilities|Select :Index State :Offline "Offline" :NotProducing "Not Producing" :Producing "Producing")))))

(event Custom|On%20Sound%20Source%20Ready
  (params (SoundWave :type Sound%20Wave%20Object%20Reference))
  (bind _audio (Variables|Default|GetAudio))
  ;[0 0.978 1] VideoCoreMediaReceiver Callbacks
  ;;[1 0.07292 0.4745] audio component setup
  (Utilities|IsValid _audio
    (:Is%20Valid
      (Audio|Components|Audio|SetSound _audio SoundWave)
      (Audio|Components|Audio|Play _audio 0.0))
    (:Is%20Not%20Valid
      (Class|DDBlueprintLibrary|LogWarning "Audio source ready but no Audio component supplied"))))

(event Custom|Mcast%20Sender%20Started%20Stream%20Produce
  (params (clientId :type String) (streamId :type String) (streamHint :type String) (kind :type EMediaTrackKind%20Enum :default "Unknown"))
  ;[1 1 1] mplayer handling
  ;;[0 0.7035 1] start produce -> start consume (sync ON only)
  (if (Utilities|Enum|NotEqual(Enum) clientId (Variables|Default|GetsenderClientId))
    (Class|DDBlueprintLibrary|LogWarning "Produce started -- client IDs don't match, overwrote"))
  (Variables|Default|SetsenderClientId clientId)
  (CallFunction|StartConsume streamHint kind))

(event Custom|Setup%20Media%20Receiver%20Callbacks
  (bind _mediareceiver (Variables|Default|GetmediaReceiver))
  ;[0 0.978 1] VideoCoreMediaReceiver Callbacks
  (EventDispatchers|BindEventtoOnSoundSourceReady _mediareceiver (delegate Custom|On%20Sound%20Source%20Ready))
  (EventDispatchers|BindEventtoOnStreamingStarted _mediareceiver (delegate Custom|On%20Streaming%20Started))
  (EventDispatchers|BindEventtoOnClientStateChanged _mediareceiver (delegate Custom|On%20Client%20State%20Changed))
  (EventDispatchers|BindEventtoOnStreamingStopped _mediareceiver (delegate Custom|On%20Streaming%20Stopped)))

(event Custom|On%20Streaming%20Stopped
  (params (ProducerId :type String) (Kind :type EMediaTrackKind%20Enum :default "Unknown") (Reason :type String))
  ;[0 0.978 1] VideoCoreMediaReceiver Callbacks
  (Class|DDBlueprintLibrary|LogWarning (Utilities|String|ToString(Text) (Utilities|Text|FormatText "Streaming stopped for {id}, reason: {reason}" ProducerId Reason))))

(event EventBeginPlay
  (CallFunction|CreateRtcObjects)
  (Utilities|SwitchbyRole))

(event EventTick
  (params (DeltaSeconds :type Float%20%28single-precision%29)))

(fn CreateRtcObjects
  (bind _self self)
  (bind _returnvalue (Game|ConstructObjectfromClass "/Script/VideoCoreRTC.VideoCoreMediaSender" _self))
  (Variables|Default|SetmediaSender _returnvalue)
  (CallFunction|SetupMediaSenderCallbacks)
  (bind _returnvalue_2 (Game|ConstructObjectfromClass "/Script/VideoCoreRTC.VideoCoreMediaReceiver" _self))
  (Variables|Default|SetmediaReceiver _returnvalue_2)
  (CallFunction|SetupMediaReceiverCallbacks))

(fn GetRole
  (bind _asplayer_controller (Utilities|Casting|CastToPlayerController (CallFunction|GetMyTopOwner))
    (:then
      (return (select (== _asplayer_controller (Game|GetPlayerController 0)) "NewEnumerator0" "NewEnumerator1")))
    (:CastFailed
      (return "NewEnumerator2"))))

(fn GetMyTopOwner
  (bind _output_get (LocalVariables|SetlastOwner (Components|GetOwner)))
  (while (and (Utilities|IsValid _output_get) (Utilities|IsValid (Components|GetOwner _output_get)))
    (LocalVariables|SetlastOwner (Components|GetOwner _output_get)))
  (return (LocalVariables|GetlastOwner)))

(fn Init
  (params (rtcSignaling :type Video%20Core%20Signaling%20Component%20Object%20Reference))
  (Variables|Default|SetrtcSignaling rtcSignaling)
  (Utilities|SwitchbyRole
    (:Sender
      (bind _returnvalue (Class|VideoCoreMediaSender|Init (Variables|Default|GetmediaSender) rtcSignaling))
      (switch Utilities|FlowControl|Switch|SwitchonESignalingClientState (Variables|/Script/VideoCoreRTC.VideoCoreSignalingComponent|Getstate rtcSignaling)
        (:NotConnected
          (CallFunction|SetupSignalingCallbacks rtcSignaling :!label _label))
        (:Connecting
          (goto _label))
        (:Connected
          (CallFunction|UpdateClientId)))
      (Utilities|SwitchonSendRecvSync
        (:Sync%20ON
          (return _returnvalue))
        (:Sync%20OFF
          _)))
    (:Receiver
      _)
    (:Unowned
      _))
  (Class|VideoCoreMediaReceiver|Init (Variables|Default|GetmediaReceiver) rtcSignaling)
  (switch Utilities|FlowControl|Switch|SwitchonESignalingClientState (Variables|/Script/VideoCoreRTC.VideoCoreSignalingComponent|Getstate rtcSignaling)
    (:NotConnected
      (CallFunction|SetupSignalingCallbacks rtcSignaling :!label _label_2))
    (:Connecting
      (goto _label_2))
    (:Connected
      (CallFunction|ValidateStreamState "Audio")
      (CallFunction|ValidateStreamState "Video")))
  (return true))

(fn StartProduce
  (params (kind :type EMediaTrackKind%20Enum :default "Unknown") (renderTarget :type Texture%20Render%20Target%202D%20Object%20Reference) (frameSize :type Int%20Point%20Structure) (minBitrate :type Integer) (streamHint :type String))
  (bind _mediasender (Variables|Default|GetmediaSender))
  (Utilities|SwitchbyRole
    (:Sender
      (Utilities|IsValid (Variables|Default|GetmediaSender)
        (:Is%20Valid
          (Variables|/Script/VideoCoreRTC.VideoCoreMediaSender|SetFrameSize _mediasender frameSize)
          (CallFunction|AddBitrate _mediasender minBitrate)
          (Variables|/Script/VideoCoreRTC.VideoCoreMediaSender|SetRenderTarget _mediasender renderTarget)
          (CallFunction|SetStreamHint streamHint kind)
          (bind _returnvalue (Class|VideoCoreMediaSender|Produce (Variables|Default|GetmediaSender) streamHint kind))
          (return _returnvalue (select _returnvalue "" "MediaSender can't produce stream")))
        (:Is%20Not%20Valid
          (return false "Media Sender is invalid"))))
    (:Receiver
      _)
    (:Unowned
      _))
  (return false (Utilities|String|ToString(Text) (Utilities|Text|FormatText "Can't produce -- current actor role is not Sender ({r})" (Utilities|Role2String)))))

(fn AddBitrate
  (params (sender :type Video%20Core%20Media%20Sender%20Object%20Reference) (bitrate :type Integer))
  (bind _bitrates (Variables|/Script/VideoCoreRTC.VideoCoreMediaSender|GetBitrates sender))
  (if (not (Utilities|Array|ContainsItem _bitrates bitrate))
    (Utilities|Array|Add _bitrates bitrate)))

(fn StartConsume
  (params (streamHint :type String) (kind :type EMediaTrackKind%20Enum :default "Video"))
  (bind _mediareceiver (Variables|Default|GetmediaReceiver))
  (bind _senderclientid (Variables|Default|GetsenderClientId))
  (Utilities|SwitchbyRole
    (:Sender
      (Utilities|SwitchonSendRecvSync
        (:Sync%20ON
          (Class|DDBlueprintLibrary|LogError "Sender can't consume"))
        (:Sync%20OFF
          (if (not (Utilities|Array|IsEmpty (Variables|Default|GetsenderClientId))) :!label _label
            (switch Utilities|FlowControl|Switch|SwitchonEMediaTrackKind kind
              (:Unknown
                (Class|DDBlueprintLibrary|LogError "Unsupported stream type to consume" :!label _label_2))
              (:Audio
                (Variables|/Script/VideoCoreRTC.VideoCoreMediaReceiver|SetaudioProducerId _mediareceiver streamHint)
                (Class|VideoCoreMediaReceiver|Consume _mediareceiver _senderclientid :!label _label_3)
                (Class|DDBlueprintLibrary|LogTrace (Utilities|String|ToString(Text) (Utilities|Text|FormatText "Will consume from {cid}" _senderclientid))))
              (:Video
                (Variables|/Script/VideoCoreRTC.VideoCoreMediaReceiver|SetvideoProducerId _mediareceiver streamHint)
                (goto _label_3))
              (:Data
                (goto _label_2)))
            (else
              (Class|DDBlueprintLibrary|LogError "Can't consume -- clienId is empty"))))))
    (:Receiver
      (goto _label))
    (:Unowned
      (goto _label))))

(fn StopConsume
  (Utilities|SwitchbyRole
    (:Sender
      (Utilities|SwitchonSendRecvSync
        (:Sync%20OFF
          _)))
    (:Receiver
      _)
    (:Unowned
      _))
  (Class|VideoCoreMediaReceiver|Stop (Variables|Default|GetmediaReceiver))
  (Class|DDBlueprintLibrary|LogTrace "Stop consume"))

(fn GetLocalRenderTexture
  (Utilities|SwitchbyRole
    (:Sender
      (Utilities|SwitchonSendRecvSync
        (:Sync%20ON
          (return (Variables|/Script/VideoCoreRTC.VideoCoreMediaSender|GetRenderTarget (Variables|Default|GetmediaSender))))
        (:Sync%20OFF
          _)))
    (:Receiver
      _)
    (:Unowned
      _))
  (return (Class|VideoCoreMediaReceiver|GetVideoTexture (Variables|Default|GetmediaReceiver))))

(fn GetSenderRenderTarget
  (Utilities|SwitchbyRole
    (:Sender
      (return (Variables|/Script/VideoCoreRTC.VideoCoreMediaSender|GetRenderTarget (Variables|Default|GetmediaSender))))
    (:Receiver
      _)
    (:Unowned
      _))
  (return 0))

(fn StopProduce
  (Class|VideoCoreMediaSender|Stop (Variables|Default|GetmediaSender) "Video"))

(fn UpdateClientId
  (bind _output_get (Variables|Default|SetsenderClientId (Variables|/Script/VideoCoreRTC.VideoCoreSignalingComponent|GetclientId (Variables|Default|GetrtcSignaling))))
  (CallFunction|ServerSetSenderClientId _output_get))

(fn SetStreamHint
  (params (hint :type String) (trackKind :type EMediaTrackKind%20Enum :default "Unknown"))
  (switch Utilities|FlowControl|Switch|SwitchonEMediaTrackKind trackKind
    (:Audio
      (Variables|StreamHints|SetaudioStreamHint hint))
    (:Video
      (Variables|StreamHints|SetvideoStreamHint hint)))
  (if (not (Networking|IsServer))
    (CallFunction|ServerSetStreamHint hint trackKind)))

(fn UpdateTrackState
  (params (kind :type EMediaTrackKind%20Enum :default "Unknown") (state :type EMediaTrackState%20Enum :default "Unknown"))
  (switch Utilities|FlowControl|Switch|SwitchonEMediaTrackKind kind
    (:Audio
      (Variables|SenderStreamState|SetaudioSenderTrackState state))
    (:Video
      (Variables|SenderStreamState|SetvideoSenderTrackState state)))
  (if (not (Networking|IsServer))
    (CallFunction|ServerSetTrackState kind state)))

(fn GetStreamHint
  (params (kind :type EMediaTrackKind%20Enum :default "Unknown"))
  (switch Utilities|FlowControl|Switch|SwitchonEMediaTrackKind kind
    (:Audio
      (return (Variables|StreamHints|GetaudioStreamHint)))
    (:Video
      (return (Variables|StreamHints|GetvideoStreamHint)))))

(fn ValidateStreamState
  (params (kind :type EMediaTrackKind%20Enum :default "Unknown"))
  (bind _state (CallFunction|GetSenderTrackState kind))
  (bind _state_2 (CallFunction|ReceiverGetTrackState kind))
  (if (Utilities|Enum|NotEqual(Enum) _state_2 _state)
    (Class|DDBlueprintLibrary|LogTrace (Utilities|String|ToString(Text) (Utilities|Text|FormatText "STREAM STATES DIFFER -- {s1} {s2} --- START CONSUME" (Utilities|Select :Index _state_2 :Unknown "unknown" :Ended "ended" :Initializing "initializing" :Live "live") (Utilities|Select :Index _state :Unknown "unknown" :Ended "ended" :Initializing "initializing" :Live "live"))))
    (CallFunction|StartConsume (CallFunction|GetStreamHint kind) kind)))

(fn GetSenderTrackState
  (params (kind :type EMediaTrackKind%20Enum :default "Unknown"))
  (switch Utilities|FlowControl|Switch|SwitchonEMediaTrackKind kind
    (:Audio
      (return (Variables|SenderStreamState|GetaudioSenderTrackState)))
    (:Video
      (return (Variables|SenderStreamState|GetvideoSenderTrackState)))))

(fn ReceiverGetTrackState
  (params (kind :type EMediaTrackKind%20Enum :default "Unknown"))
  (return (Class|VideoCoreMediaReceiver|GetTrackState (Variables|Default|GetmediaReceiver) kind)))