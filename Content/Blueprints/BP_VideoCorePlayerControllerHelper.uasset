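; Player controller helper component for VideoCore, handling multiplayer control of in-world video planes.
; Polls local and server NDI sources, relays plane edits and save/load through server events, and auto-loads a saved game from the command line.
; Tick drives left-mouse plane grabbing via relative transforms, adds right-mouse to possess the grabbed plane with a delayed release lock, and keeps NDI/RTC broadcasters on the pawn's camera.
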(event Custom|Client%20On%20Plane%20Spawned
  (params (planeName :type String))
  ;[1 0.1593 0.9455] multiplayer plane spawning
  ;;[1 1 1] Calling user callback passed when SpawnNewPlane was called
  (Class|PlayerControllerHelper|CallUseronNewPlaneSpawned planeName))

(event Custom|Server%20Set%20Plane%20Pivot%20Point
  (params (plane :type BP%20Plane%20Base%20Object%20Reference) (pp :type Vector%202D%20Structure))
  ;[1 1 1] set plane pivot point
  (Default|SetPivotPoint plane pp))

(event Custom|Server%20Set%20Plane%20Keying
  (params (plane :type BP%20Plane%20Base%20Object%20Reference) (alphaCutoffMin :type Float%20%28single-precision%29) (alphaCutoffMax :type Float%20%28single-precision%29) (alphaExp :type Float%20%28single-precision%29) (despillCutoffMax :type Float%20%28single-precision%29) (despillExp :type Float%20%28single-precision%29) (keyColor :type Linear%20Color%20Structure) (alphaCutoffMin2 :type Float%20%28single-precision%29) (alphaCutoffMax2 :type Float%20%28single-precision%29) (alphaExp2 :type Float%20%28single-precision%29) (despillCutoffMax2 :type Float%20%28single-precision%29) (despillExp2 :type Float%20%28single-precision%29) (keyColor2 :type Linear%20Color%20Structure))
  ;[1 1 1] mplayer texture parameters update handling
  (Utilities|IsValid plane
    (:Is%20Valid
      (Default|SetKeyingParams plane alphaCutoffMin alphaCutoffMax alphaExp despillCutoffMax despillExp keyColor alphaCutoffMin2 alphaCutoffMax2 alphaExp2 despillCutoffMax2 despillExp2 keyColor2))))

(event Custom|Server%20Set%20Autorotate%20Axis
  (params (plane :type BP%20Plane%20Base%20Object%20Reference) (axis :type Vector))
  ;[1 1 1] A/R Axis
  (Variables|/VideoCore/Blueprints/BP_PlaneBase.BP_PlaneBase_C|SetautorotateAxis plane axis))

(event Custom|Server%20Set%20Plane%20Visibility
  (params (visible :type Boolean) (applyCounterpart :type Boolean) (plane :type BP%20Plane%20Base%20Object%20Reference))
  (bind _counterpart (CallFunction|FindCounterpartPlane plane))
  (bind _returnvalue (not visible))
  ;[1 1 1] plane UI controls server-side
  (Rendering|SetActorHiddenInGame plane _returnvalue)
  (if (and applyCounterpart (Utilities|IsValid _counterpart))
    (Rendering|SetActorHiddenInGame _counterpart _returnvalue)))

(event Custom|Server%20Toggle%20Plane%20Playback
  (params (applyCounterpart :type Boolean) (plane :type BP%20Plane%20Base%20Object%20Reference))
  ;[1 1 1] plane UI controls server-side
  (Utilities|Casting|CastToBP_RecordedPlane plane)
  (if applyCounterpart
    (Utilities|Casting|CastToBP_RecordedPlane (CallFunction|FindCounterpartPlane plane))))

(event Custom|Server%20Set%20Plane%20Auto%20Rotate
  (params (isAutorotate :type Boolean) (applyCounterpart :type Boolean) (plane :type BP%20Plane%20Base%20Object%20Reference))
  (bind _counterpart (CallFunction|FindCounterpartPlane plane))
  ;[1 1 1] plane UI controls server-side
  (Variables|/VideoCore/Blueprints/BP_PlaneBase.BP_PlaneBase_C|SetisAutoRotate plane isAutorotate)
  (if (and applyCounterpart (Utilities|IsValid _counterpart))
    (Variables|/VideoCore/Blueprints/BP_PlaneBase.BP_PlaneBase_C|SetisAutoRotate _counterpart isAutorotate)))

(event Custom|Server%20Delete%20Plane
  (params (applyCounterpart :type Boolean) (plane :type BP%20Plane%20Base%20Object%20Reference))
  (bind _counterpart (CallFunction|FindCounterpartPlane plane))
  ;[1 1 1] plane UI controls server-side
  (Actor|DestroyActor plane)
  (if applyCounterpart
    (Utilities|IsValid _counterpart
      (:Is%20Valid
        (Actor|DestroyActor _counterpart)))))

(event Custom|Client%20Received%20Remote%20Ndi%20Sources
  (params (sources :type Array%20of%20NDI%20Connection%20Information%20Structures))
  ;[1 1 1] handling requesting server-side NDI planes
  (if (not (Networking|IsServer))
    (Variables|NDIPlanes|SetserverNdiSources sources)))

(event Custom|Server%20Set%20Plane%20Owner
  (params (plane :type BP%20Plane%20Base%20Object%20Reference) (newOwner :type Player%20Controller%20Object%20Reference))
  ;[1 0.3152 0.6139] plane ownership control
  (Actor|SetOwner plane newOwner))

(event Custom|Server%20Request%20Remote%20Ndi%20Sources
  ;[1 1 1] handling requesting server-side NDI planes
  (CallFunction|ClientReceivedRemoteNdiSources (Variables|NDIPlanes|GetndiSources)))

(event Custom|Server%20NDI%20Plane%20Set%20Source
  (params (plane :type BP%20Ndi%20Plane%20Object%20Reference) (source :type NDI%20Connection%20Information%20Structure))
  ;[1 1 1] server-side NDI plane control
  (Default|SetNDISource plane source))

(event Custom|Client%20On%20Possessed%20Pawn
  ;[0 1 0.8309] pawn posession handling
  (Default|CallOnPawnPossessedHandler))

(event Custom|Server%20NDI%20Plane%20Stop%20Streaming
  (params (plane :type BP%20Ndi%20Plane%20Object%20Reference))
  ;[1 1 1] server-side NDI plane control
  (Default|StopStreaming plane true))

(event Custom|Server%20NDI%20Plane%20Start%20Streaming
  (params (plane :type BP%20Ndi%20Plane%20Object%20Reference) (source :type NDI%20Connection%20Information%20Structure))
  ;[1 1 1] server-side NDI plane control
  (Default|SetNDISource plane source)
  (Default|StopStreaming plane true)
  (Default|StartStreaming plane))

(event Custom|Server%20Possess
  (params (pawn :type Pawn%20Object%20Reference))
  (bind _playercontroller (CallFunction|GetOwnerPlayerController))
  ;[0 1 0.8309] pawn posession handling
  (Pawn|UnPossess _playercontroller)
  (Pawn|Possess _playercontroller pawn)
  (Utilities|FlowControl|Delay 0.1)
  (CallFunction|ClientonPossessedPawn))

(event Custom|Server%20Save%20Game
  (params (fileName :type String))
  ;[1 0.1342 0] save/load game on server
  (bind _result (CallFunction|SaveVideoCoreGame fileName false))
  (Class|DDBlueprintLibrary|LogTrace (Utilities|String|ToString(Text) (Utilities|Text|FormatText "Server game save res: {r}" _result))))

(event Custom|Server%20Load%20Game
  (params (fileName :type String))
  ;[1 0.1342 0] save/load game on server
  (bind _success (CallFunction|LoadVideoCoreGame fileName))
  (Class|DDBlueprintLibrary|LogTrace (Utilities|String|ToString(Text) (Utilities|Text|FormatText "Server game load res: {r}" _success))))

(event Custom|Server%20Set%20Plane%20Orientation
  (params (plane :type BP%20Plane%20Base%20Object%20Reference) (orientation :type EVideoCorePlaneOrientation%20Enum :default "HorizontalDefault"))
  ;[1 1 1] set orientation
  (Default|SetOrientation plane orientation))

(event Custom|Server%20Set%20Autounfreeze
  (params (plane :type BP%20Ndi%20Plane%20Object%20Reference) (autoUnfreeze :type Boolean))
  ;[1 1 1] autounfreeze
  (Variables|/VideoCore/Blueprints/BP_NdiPlane.BP_NdiPlane_C|SetautoUnfreeze plane autoUnfreeze))

(event Custom|Server%20Set%20Plane%20Tint%20Color
  (params (plane :type BP%20Plane%20Base%20Object%20Reference) (color :type Vector))
  ;[1 1 1] set tint color
  (Default|SetTintColor plane color))

(event Custom|Server%20Set%20Actor%20Transform
  (params (actor :type Actor%20Object%20Reference) (t :type Transform))
  ;[0.3558 1 0] TODO: REQUIRES FIX. temporarily forward call to player controller
  ; server-side actor transform update
  (bind _asplayer_controller_gh_base (Utilities|Casting|CastToPlayerController_GH_Base (CallFunction|GetOwnerPlayerController)))
  (Default|ServerSetActorTransform _asplayer_controller_gh_base actor t))

(event Custom|Server%20Set%20Plane%20Label
  (params (plane :type BP%20Plane%20Base%20Object%20Reference) (label :type String))
  ;[1 1 1] handling mplayer plane label control
  (Variables|/VideoCore/Blueprints/BP_PlaneBase.BP_PlaneBase_C|SetplaneLabelString plane label))

(event Custom|Fetch%20NDI%20Sources
  (bind _returnvalue (Class|NDIIOLibrary|GetNDISourceCollection))
  ;[1 1 1] NDI sources fetching
  (if (!= (Utilities|Array|Length _returnvalue) (Utilities|Array|Length (Variables|NDIPlanes|GetndiSources)))
    (Variables|NDIPlanes|SetndiSources _returnvalue)
    (Default|CallOnNdiSourceListUpdated))
  (if (Networking|IsServer)
    _
    (else
      (CallFunction|ServerRequestRemoteNdiSources)))
  (Utilities|FlowControl|Delay 3.0)
  (CallFunction|FetchNDISources))

(event Custom|Server%20Set%20Plane%20Label%20Visibility
  (params (plane :type BP%20Plane%20Base%20Object%20Reference) (isVisible :type Boolean))
  ;[1 1 1] handling mplayer plane label control
  (Default|SetPlaneLabelVisibility plane isVisible))

(event Custom|Release%20TP%20Control%20Lock
  ;[1 0 0] handle plane grabbing
  ;;[1 0.4278 0.1332] this is needed when releasing TP control -- after pawn unpossessing
  (Utilities|FlowControl|Delay 0.2)
  (Variables|PlaneDrag|SettpControlReleaseLock false))

(event Custom|Server%20Set%20Plane%20Crop
  (params (plane :type BP%20Plane%20Base%20Object%20Reference) (crop :type Two%20Vectors%20Structure))
  ;[1 1 1] mplayer texture parameters update handling
  (CallFunction|McastSetPlaneCrop plane crop))

(event Custom|Mcast%20Set%20Plane%20Crop
  (params (Target :type BP%20Plane%20Base%20Object%20Reference) (selectionNormalized :type Two%20Vectors%20Structure))
  ;[1 1 1] mplayer texture parameters update handling
  (Default|SetFrameSelection Target selectionNormalized))

(event EventBeginPlay
  ;[1 0.1057 0] begin play
  (Variables|Default|SetgamePlanes (CallFunction|GetAllPlanes))
  (CallFunction|FetchNDISources)
  (Class|NDIIOLibrary|BeginBroadcastingActiveViewport)
  (CallFunction|CheckStartupArgs))

(event EventTick
  (params (DeltaSeconds :type Float%20%28single-precision%29))
  (Utilities|FlowControl|Sequence
    (:then_0
      ;[1 0 0] handle plane grabbing
      (if (Game|Player|IsInputKeyDown (CallFunction|GetOwnerPlayerController) "LeftMouseButton")
        (if (Game|Player|IsInputKeyDown (CallFunction|GetOwnerPlayerController) "RightMouseButton")
          (if (Variables|PlaneDrag|GettpControl)
            (CallFunction|HandleKeyStrokes :!label _label)
            (else
              (PlaneDrag|ActivateTPControl true)))
          (elif (Variables|PlaneDrag|GettpControl)
            (PlaneDrag|ActivateTPControl false)
            (elif (not (Variables|PlaneDrag|GettpControlReleaseLock))
              (PlaneDrag|HandlePlaneGrabbing)
              (goto _label))))
        (else
          (if (Variables|PlaneDrag|GettpControl)
            (PlaneDrag|ActivateTPControl false))
          (Utilities|IsValid (Variables|PlaneDrag|GetgrabbedPlane)
            (:Is%20Valid
              (Default|SetIsGrabbed (Variables|PlaneDrag|GetgrabbedPlane) false)
              (Variables|PlaneDrag|SetgrabbedPlane 0))))))
    (:then_1
      (POVBroadcast|UpdatePawnBroadcaster))))

(event EventOnServerSpawnedPlane
  (params (plane :type Actor%20Object%20Reference))
  ;[1 0.1593 0.9455] multiplayer plane spawning
  (Utilities|IsValid plane
    (:Is%20Valid
      (bind _asbp_live_plane (Utilities|Casting|CastToBP_LivePlane plane)
        (:then
          (CallFunction|ClientonPlaneSpawned (Default|GetFullTextId _asbp_live_plane)))
        (:CastFailed
          (Class|DDBlueprintLibrary|LogError "Server spawned something other than a plane"))))
    (:Is%20Not%20Valid
      (Class|DDBlueprintLibrary|LogError "Server failed to spawn a plane"))))

(fn SpawnLivePlane
  (params (animated :type Boolean))
  (Class|PlayerControllerHelper|SpawnPlaneActor "/VideoCore/Blueprints/BP_LivePlane.BP_LivePlane_C" (CallFunction|GetSpawnTransform animated) (EventDispatchers|CreateEvent :!event OnNewPlaneSpawned)))

(fn OnNewPlaneSpawned
  (params (name :type String)))

(fn GetSpawnTransform
  (params (forAnimation :type Boolean))
  (bind _playercontroller (CallFunction|GetOwnerPlayerController))
  (bind _playercontroller_2 (CallFunction|GetOwnerPlayerController))
  (bind _returnvalue (Pawn|GetControlledPawn _playercontroller))
  (bind _returnvalue_2 (Pawn|GetControlledPawn _playercontroller_2))
  (bind _returnvalue_3 (Transformation|GetActorTransform _returnvalue_2))
  (bind _returnvalue_4 (Transformation|GetActorTransform _returnvalue))
  (bind (_location _rotation _scale) (Math|Transform|BreakTransform _returnvalue_3))
  (bind (_location_2 _rotation_2 _scale_2) (Math|Transform|BreakTransform _returnvalue_4))
  (if forAnimation
    (return (Math|Transform|MakeTransform (+ (* (Transformation|GetActorUpVector _returnvalue) 1e+02) _location_2) (Math|Rotator|MakeRotfromX (* (Math|Rotator|GetRotationXVector _rotation_2) -1.0)) _scale_2))
    (else
      ;[1 1 1] 8 meters away facing player
      (return (Math|Transform|MakeTransform (+ (* (Transformation|GetActorUpVector _returnvalue_2) -2e+02) (* (Transformation|GetActorForwardVector _returnvalue_2) 8e+02) _location) (Math|Rotator|MakeRotfromX (* (Math|Rotator|GetRotationXVector _rotation) -1.0)) _scale)))))

(fn ProbePlane
  (params (distance :type Float%20%28single-precision%29))
  (bind _playercontroller (CallFunction|GetOwnerPlayerController))
  (bind _returnvalue (Pawn|GetControlledPawn _playercontroller))
  (bind _returnvalue_2 (Transformation|GetActorLocation _returnvalue))
  (bind (_outhit _returnvalue_3) (Collision|LineTraceForObjects _returnvalue_2 (+ _returnvalue_2 (* (Transformation|GetActorForwardVector _returnvalue) distance)) (Utilities|Array|MakeArray "ObjectTypeQuery3") false (Utilities|Array|MakeArray _returnvalue) "None"))
  (if _returnvalue_3
    (bind _asbp_plane_base (Utilities|Casting|CastToBP_PlaneBase (.HitActor (Collision|BreakHitResult _outhit)))
      (:then
        (if (Default|IsPlaneDragEnabled _asbp_plane_base)
          (return _asbp_plane_base)
          (else
            _)))
      (:CastFailed
        _)))
  (return 0))

(fn HandlePlaneGrabbing
  (Utilities|IsValid (Variables|PlaneDrag|GetgrabbedPlane)
    (:Is%20Valid
      (CallFunction|ServerSetActorTransform (Variables|PlaneDrag|GetgrabbedPlane) (Math|Transform|ComposeTransforms (Variables|PlaneDrag|GetgrabTransform) (CallFunction|GetPlayerTransform))))
    (:Is%20Not%20Valid
      (bind _hitplane (PlaneDrag|ProbePlane (LocalVariables|GetgrabDistance)))
      (Utilities|IsValid _hitplane
        (:Is%20Valid
          (bind _output_get (Variables|PlaneDrag|SetgrabbedPlane _hitplane))
          (Default|SetIsGrabbed _output_get true)
          (Variables|PlaneDrag|SetgrabTransform (Math|Transform|MakeRelativeTransform (Transformation|GetActorTransform _output_get) (CallFunction|GetPlayerTransform))))))))

(fn ActivateTPControl
  (params (activate :type Boolean))
  (bind _grabbedplane (Variables|PlaneDrag|GetgrabbedPlane))
  (Class|DDBlueprintLibrary|LogTrace (Utilities|String|ToString(Text) (Utilities|Text|FormatText "SET TP CONTROL TO {b1} CURRENT {b}" activate (Variables|PlaneDrag|GettpControl))))
  (EventDispatchers|BindEventtoOnPawnPossessedHandler (EventDispatchers|CreateEvent :!event TPControlPawnPossessed))
  (if activate
    (Utilities|IsValid _grabbedplane
      (:Is%20Valid
        (Variables|PlaneDrag|SettpControlPawn (Pawn|GetControlledPawn (CallFunction|GetOwnerPlayerController)))
        (Variables|PlaneDrag|SetprePossessRotation (Transformation|GetActorRotation _grabbedplane))
        (Variables|PlaneDrag|SettpControl true)
        (Class|DDBlueprintLibrary|LogTrace "TP CONTROL SET TO TRUE")
        (CallFunction|ServerPossess (Variables|PlaneDrag|GetgrabbedPlane))))
    (else
      (Utilities|IsValid (Variables|PlaneDrag|GettpControlPawn)
        (:Is%20Valid
          (Variables|PlaneDrag|SetprePossessRotation (Transformation|GetActorRotation (Variables|PlaneDrag|GettpControlPawn)))
          (Variables|PlaneDrag|SettpControl false)
          (Variables|PlaneDrag|SettpControlReleaseLock true)
          (CallFunction|ServerPossess (Variables|PlaneDrag|GettpControlPawn)))))))

(fn TPControlPawnPossessed
  (bind _playercontroller (CallFunction|GetOwnerPlayerController))
  (Utilities|IsValid (Variables|PlaneDrag|GettpControlPawn)
    (:Is%20Valid
      (Game|Player|SetViewTargetwithBlend _playercontroller (Variables|PlaneDrag|GettpControlPawn) 0.0 "VTBlend_EaseOut" 0.0 false)
      (Pawn|SetControlRotation _playercontroller (Variables|PlaneDrag|GetprePossessRotation))
      (if (Variables|PlaneDrag|GettpControl)
        _
        (else
          (Class|DDBlueprintLibrary|LogTrace "Clear owner pawn variable")
          (Variables|PlaneDrag|SettpControlPawn 0)
          (Utilities|IsValid (Variables|PlaneDrag|GetgrabbedPlane)
            (:Is%20Valid
              (Default|SetIsGrabbed (Variables|PlaneDrag|GetgrabbedPlane) false)
              (Variables|PlaneDrag|SetgrabbedPlane 0))
            (:Is%20Not%20Valid
              _))
          (CallFunction|ReleaseTPControlLock)))
      (EventDispatchers|UnbindallEventsfromOnPawnPossessedHandler))
    (:Is%20Not%20Valid
      (Class|DDBlueprintLibrary|LogError "On Pawn Possess Callback Error: TP Control Owner Pawn is NONE"))))

(fn HandleKeyStrokes
  (bind _playercontroller (CallFunction|GetOwnerPlayerController))
  (if (Game|Player|IsInputKeyDown _playercontroller "LeftControl")
    (if (Game|Player|IsInputKeyDown _playercontroller "C")
      (CallFunction|CopyPlane (Variables|PlaneDrag|GetgrabbedPlane))
      (else
        ;[1 1 1] auto rotate
        (if (Game|Player|IsInputKeyDown _playercontroller "R")
          (Default|SetLookat (Variables|PlaneDrag|GetgrabbedPlane) (select (Variables|PlaneDrag|GettpControl) (Variables|PlaneDrag|GettpControlPawn) (Pawn|GetControlledPawn (CallFunction|GetOwnerPlayerController)))))))))

(fn CopyPlane
  (params (plane :type BP%20Plane%20Base%20Object%20Reference))
  (Class|VideoCoreFunctionLibrary|ClipboardCopy (Utilities|String|ToString(Text) (Utilities|Text|FormatText "{str1} 
{str2} 
{str3}" (Default|GetPlaneDebugString1 plane) (Default|GetPlaneDebugString2 plane) (Default|GetPlaneDebugString3 plane)))))

(fn GetSourcesNames
  (params (arr :type Array%20of%20NDI%20Connection%20Information%20Structures))
  (for _array_element arr
    (Utilities|Array|Add (LocalVariables|Geta) (.SourceName (Utilities|Struct|BreakNDIConnectionInformation _array_element))))
  (return (LocalVariables|Geta)))

(fn GetConnectionInfoforSource
  (params (sourceName :type String))
  (for _array_element (Variables|NDIPlanes|GetndiSources)
    (if (Utilities|Enum|Equal(Enum) sourceName (.SourceName (Utilities|Struct|BreakNDIConnectionInformation _array_element)))
      (return true _array_element)))
  (return false ""))

(fn GetOwnerPlayerController
  (bind _asplayer_controller (Utilities|Casting|CastToPlayerController (Components|GetOwner))
    (:then
      (return _asplayer_controller))
    (:CastFailed
      (Class|DDBlueprintLibrary|LogError "FATAL: Can't get VideoCore Helper owner player controller")
      (return 0))))

(fn SetupNDIBroadcaster
  (bind _returnvalue (Game|SpawnActorfromClass "/VideoCore/Blueprints/BP_NDI_BroadcastActor.BP_NDI_BroadcastActor_C" (Math|Transform|MakeTransform "0, 0, 0") "Undefined" (CallFunction|GetOwnerPlayerController) 0))
  (bind _output_get (Variables|Broadcast|SetpawnNdiBroadcaster _returnvalue))
  (return _output_get))

(fn UpdatePawnBroadcaster
  (bind _playercontroller (CallFunction|GetOwnerPlayerController))
  (bind _pawnndibroadcaster (Variables|Broadcast|GetpawnNdiBroadcaster))
  (bind _pawnrtcbroadcaster (Variables|Broadcast|GetpawnRtcBroadcaster))
  (bind _returnvalue (Pawn|GetControlledPawn _playercontroller))
  (bind _camera (CallFunction|GetActivePawnCamera _returnvalue))
  (Utilities|IsValid _camera
    (:Is%20Valid
      (LocalVariables|SettargetT (Transformation|GetWorldTransform _camera)))
    (:Is%20Not%20Valid
      (LocalVariables|SettargetT (Transformation|GetActorTransform _returnvalue))))
  (Utilities|FlowControl|Sequence
    (:then_0
      (Utilities|IsValid _pawnndibroadcaster
        (:Is%20Valid
          (Transformation|SetActorTransform _pawnndibroadcaster (LocalVariables|GettargetT)))))
    (:then_1
      (Utilities|IsValid _pawnrtcbroadcaster
        (:Is%20Valid
          (Transformation|SetActorTransform _pawnrtcbroadcaster (LocalVariables|GettargetT)))))))

(fn CheckStartupArgs
  (bind _returnvalue (Class|VideoCoreFunctionLibrary|GetCommandLineArgs))
  (Utilities|FlowControl|Sequence
    (:then_0
      (if (.ReturnValue (Utilities|Map|Find _returnvalue "videoCoreGame"))
        (bind _success (CallFunction|LoadVideoCoreGame (.Value (Utilities|Map|Find _returnvalue "videoCoreGame"))))
        (if _success
          (Class|DDBlueprintLibrary|LogTrace (Utilities|String|ToString(Text) (Utilities|Text|FormatText "Auto-load game {g}" (.Value (Utilities|Map|Find _returnvalue "videoCoreGame")))))
          (else
            (Class|DDBlueprintLibrary|LogError (Utilities|String|ToString(Text) (Utilities|Text|FormatText "Failed to auto-load game {g}" (.Value (Utilities|Map|Find _returnvalue "videoCoreGame")))))))))))

(fn SetupRTCBroadcaster
  (params (frameSize :type Int%20Point%20Structure) (bitrate :type Integer))
  (bind _returnvalue (Game|SpawnActorfromClass "/VideoCore/Blueprints/BP_RtcBroadcastActor.BP_RtcBroadcastActor_C" (Math|Transform|MakeTransform "0, 0, 0") "Undefined" (CallFunction|GetOwnerPlayerController) 0))
  (Utilities|IsValid _returnvalue
    (:Is%20Valid
      (bind _output_get (Variables|Broadcast|SetpawnRtcBroadcaster _returnvalue))
      (Variables|/Script/VideoCoreRTC.VideoCoreMediaSender|SetFrameSize (Variables|/VideoCore/Blueprints/BP_RtcBroadcastActor.BP_RtcBroadcastActor_C|GetrtcSender _output_get) frameSize)
      (Utilities|Array|Add (Variables|/Script/VideoCoreRTC.VideoCoreMediaSender|GetBitrates (Variables|/VideoCore/Blueprints/BP_RtcBroadcastActor.BP_RtcBroadcastActor_C|GetrtcSender _output_get)) bitrate)
      (return _output_get))
    (:Is%20Not%20Valid
      (Class|DDBlueprintLibrary|LogWarning "Failed to spawn broadcast actor"))))