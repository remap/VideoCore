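; Plane actor that displays a remote RTC client's video stream and plays its audio, with a label showing the client's name.
; On BeginPlay it creates a VideoCoreMediaReceiver that auto-consumes the client's streams through the signaling component.
; Receiver events feed the sound wave to the audio component and toggle a material parameter enabling the video texture, with a proxy texture also set.
; It extends the parent's debug string with track states and receiver stats.
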(event Custom|Initialize%20RTC%20Plane
  ;[1 0.7449 0] initialization
  (Utilities|IsValid (CallFunction|GetVideoCoreSignalingComponent)
    (:Is%20Valid
      (CallFunction|SetupRTCMediaReceiver))
    (:Is%20Not%20Valid
      (Class|DDBlueprintLibrary|LogError "VideoCore siganling component is not found")
      (Actor|Tick|SetActorTickEnabled false))))

(event Custom|On%20Sound%20Source%20Ready
  (params (SoundWave :type Sound%20Wave%20Object%20Reference))
  (bind _audio (Variables|Default|GetAudio))
  ;[1 1 1] setup RTC events bindings
  ;;[1 0.07292 0.4745] audio component setup
  (Audio|Components|Audio|SetSound _audio SoundWave)
  (Audio|Components|Audio|Play _audio 0.0))

(event Custom|On%20Streaming%20Started
  (params (ProducerId :type String) (Kind :type EMediaTrackKind%20Enum :default "Unknown"))
  (bind _clientid (Variables|RTCConsume|GetclientId))
  (bind _clientinfo (CallFunction|FindRTCClient _clientid))
  (bind _clientname (Utilities|Struct|BreakVideoCoreMediaServerClientInfo _clientinfo))
  ;[1 1 1] setup RTC events bindings
  (Class|DDBlueprintLibrary|LogTrace (Utilities|String|ToString(Text) (Utilities|Text|FormatText "Started consuming from {id}" ProducerId)))
  (CallFunction|SetPlaneLabelString _clientname)
  (CallFunction|SetPlaneLabelVisibility (not (Utilities|Array|IsEmpty _clientname)))
  (switch Utilities|FlowControl|Switch|SwitchonEMediaTrackKind Kind
    (:Video
      (CallFunction|SetVideoTextureEnabled true))))

(event Custom|Setup%20RTC%20Media%20Receiver
  ;[1 1 1] setup RTC media receiver
  (bind _returnvalue (Game|ConstructObjectfromClass "/Script/VideoCoreRTC.VideoCoreMediaReceiver" self))
  (bind _output_get (Variables|VideoCoreRTC|SetvideoCoreMediaReceiver _returnvalue))
  (Variables|/Script/VideoCoreRTC.VideoCoreMediaReceiver|SetclientId _output_get (Variables|RTCConsume|GetclientId))
  (Variables|/Script/VideoCoreRTC.VideoCoreMediaReceiver|SetAutoConsume _output_get true)
  (Variables|/Script/VideoCoreRTC.VideoCoreMediaReceiver|SetaudioProducerId (Variables|VideoCoreRTC|GetvideoCoreMediaReceiver) (Variables|RTCConsume|GetaudioStreamHint_0))
  (Variables|/Script/VideoCoreRTC.VideoCoreMediaReceiver|SetvideoProducerId (Variables|VideoCoreRTC|GetvideoCoreMediaReceiver) (Variables|RTCConsume|GetvideoStreamHint))
  (CallFunction|SetupRTCBindings)
  (Class|VideoCoreMediaReceiver|Init _output_get (CallFunction|GetVideoCoreSignalingComponent))
  (CallFunction|SetupMaterialInstance))

(event Custom|Setup%20RTC%20Bindings
  (bind _videocoremediareceiver (Variables|VideoCoreRTC|GetvideoCoreMediaReceiver))
  ;[1 1 1] setup RTC events bindings
  (EventDispatchers|BindEventtoOnSoundSourceReady _videocoremediareceiver (delegate Custom|On%20Sound%20Source%20Ready))
  (EventDispatchers|BindEventtoOnStreamingStarted _videocoremediareceiver (delegate Custom|On%20Streaming%20Started))
  (EventDispatchers|BindEventtoOnClientStateChanged _videocoremediareceiver (delegate Custom|On%20Client%20State%20Changed))
  (EventDispatchers|BindEventtoOnStreamingStopped _videocoremediareceiver (delegate Custom|On%20Streaming%20Stopped)))

(event Custom|On%20Client%20State%20Changed
  (params (State :type EClientState%20Enum :default "Offline"))
  ;[1 1 1] setup RTC events bindings
  (Class|DDBlueprintLibrary|LogTrace (Utilities|String|ToString(Text) (Utilities|Text|FormatText "Client state changed: {st}" (Utilities|Select :Index State :Offline "Offline" :NotProducing "Not Producing" :Producing "Producing")))))

(event Custom|On%20Streaming%20Stopped
  (params (ProducerId :type String) (Kind :type EMediaTrackKind%20Enum :default "Unknown") (Reason :type String))
  ;[1 1 1] setup RTC events bindings
  (Class|DDBlueprintLibrary|LogWarning (Utilities|String|ToString(Text) (Utilities|Text|FormatText "Streaming stopped for {id}, reason: {reason}" ProducerId Reason)))
  (switch Utilities|FlowControl|Switch|SwitchonEMediaTrackKind Kind
    (:Video
      (CallFunction|SetVideoTextureEnabled false))))

(event EventBeginPlay
  (|CallParentFunction)
  (CallFunction|InitializeRTCPlane))

(event Collision|EventActorBeginOverlap
  (params (OtherActor :type Actor%20Object%20Reference))
  (|CallParentFunction OtherActor) ; This node is disabled and will not be called.\nDrag off pins to build functionality.
)

(event EventTick
  (params (DeltaSeconds :type Float%20%28single-precision%29))
  (|CallParentFunction DeltaSeconds) ; This node is disabled and will not be called.\nDrag off pins to build functionality.
)

(fn ConstructionScript
  (|CallParentFunction)
  (CallFunction|SetupMaterialInstance))

(fn SetupMaterialInstance
  (Rendering|Material|SetTextureParameterValue (Variables|Default|GetmyMaterialInstance) "Video Texture" (Class|VideoCoreMediaReceiver|GetVideoTexture (Variables|VideoCoreRTC|GetvideoCoreMediaReceiver)))
  (Rendering|Material|SetTextureParameterValue (Variables|Default|GetmyMaterialInstance) "Proxy Texture" (Variables|VideoCoreRTC|GetproxyTexture)))

(fn SetVideoTextureEnabled
  (params (enabled :type Boolean))
  (Rendering|Material|SetScalarParameterValue (Variables|Default|GetmyMaterialInstance) "Enable Video Texture" (select enabled 1.0 0.0) :!class /Script/Engine.MaterialInstanceDynamic))

(fn GetPlaneDebugString3
  (bind _videocoremediareceiver (Variables|VideoCoreRTC|GetvideoCoreMediaReceiver))
  (bind _returnvalue (Class|VideoCoreMediaReceiver|GetStats _videocoremediareceiver))
  (bind (_audiolevel _typingnoisedetected _voicedetected _samplesreceived _audiobuffersize _audiobufferstate _videocontenthint _framesreceived) (Utilities|Struct|BreakVideoCoreMediaStreamStatistics _returnvalue))
  (bind (_x _y) (Utilities|Struct|BreakIntPoint _audiobufferstate))
  (return (Utilities|String|ToString(Text) (Utilities|Text|FormatText "{s} 
client ID: {clientId} 
video ID: {vid} 
audio ID: {aid} 
client status: {status} 
{audioStr} 
{videoStr} 
audio level: {al} 
typing: {typ} 
voice: {vo} 
asamples: {asam} 
abuffer: {abuf} ({size}/{capacity}) 
video content: {vcon} 
vframes: {vfram}" (|CallParentFunction) (Variables|/Script/VideoCoreRTC.VideoCoreMediaReceiver|GetclientId _videocoremediareceiver) (Variables|/Script/VideoCoreRTC.VideoCoreMediaReceiver|GetvideoProducerId _videocoremediareceiver) (Variables|/Script/VideoCoreRTC.VideoCoreMediaReceiver|GetaudioProducerId _videocoremediareceiver) (Utilities|Select :Index (Class|VideoCoreMediaReceiver|GetRemoteClientState _videocoremediareceiver) :Offline "Offline" :NotProducing "Not Producing" :Producing "Producing") (Debugging|DebugStringforTrack "Audio" _videocoremediareceiver) (Debugging|DebugStringforTrack "Video" _videocoremediareceiver) _audiolevel _typingnoisedetected _voicedetected _samplesreceived _audiobuffersize _x _y _videocontenthint _framesreceived))))

(fn DebugStringforTrack
  (params (kind :type EMediaTrackKind%20Enum :default "Audio") (rtcReceiver :type Video%20Core%20Media%20Receiver%20Object%20Reference))
  (return (Utilities|Text|FormatText "has {tt} - {has} state {s} enabled {e}" (Utilities|Select :Index kind :Unknown "" :Audio "Audio" :Video "Video" :Data "") (Class|VideoCoreMediaReceiver|HasTrackOfType rtcReceiver kind) (Utilities|Select :Index (Class|VideoCoreMediaReceiver|GetTrackState rtcReceiver kind) :Unknown "Unknown" :Ended "Ended" :Initializing "" :Live "Live") (Class|VideoCoreMediaReceiver|GetIsTrackEnabled rtcReceiver kind))))