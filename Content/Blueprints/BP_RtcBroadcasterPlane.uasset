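; Broadcaster plane actor that streams a scene capture as video over RTC through a VideoCore media sender.
; On BeginPlay it creates a render target if needed, feeds it from the SceneCaptureComponent2D and shows it on its material with updated keying parameters.
; It then builds the sender from that target and its stream settings, initializes it with VideoCore signaling, and binds callbacks that log production start, failure and stop.
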(event Custom|Setup%20Callbacks
  (bind _rtcsender (Variables|Default|GetrtcSender))
  ;[1 0.06771 0.06771] VideoCoreMediaSender Callbacks
  (EventDispatchers|BindEventtoOnStartProducing _rtcsender (delegate Custom|On%20Start%20Producing%20Stream))
  (EventDispatchers|BindEventtoOnProduceFailure _rtcsender (delegate Custom|On%20Produce%20Failure))
  (EventDispatchers|BindEventtoOnStoppedProducing _rtcsender (delegate Custom|On%20Stopped%20Producing%20Stream)))

(event Custom|On%20Start%20Producing%20Stream
  (params (StreamId :type String) (Kind :type EMediaTrackKind%20Enum :default "Unknown"))
  ;[1 0.06771 0.06771] VideoCoreMediaSender Callbacks
  (Class|DDBlueprintLibrary|LogInfo (Utilities|String|ToString(Text) (Utilities|Text|FormatText "Started producing stream of type {type} id {id}" (Utilities|TrackKind2String Kind) StreamId))))

(event Custom|On%20Produce%20Failure
  (params (StreamId :type String) (Kind :type EMediaTrackKind%20Enum :default "Unknown") (Reason :type String))
  ;[1 0.06771 0.06771] VideoCoreMediaSender Callbacks
  (Class|DDBlueprintLibrary|LogError (Utilities|String|ToString(Text) (Utilities|Text|FormatText "Failed to produce stream {id} ({type}): {reason}" StreamId (Utilities|TrackKind2String Kind) Reason))))

(event Custom|On%20Stopped%20Producing%20Stream
  (params (StreamId :type String) (Kind :type EMediaTrackKind%20Enum :default "Unknown") (Reason :type String))
  ;[1 0.06771 0.06771] VideoCoreMediaSender Callbacks
  (Class|DDBlueprintLibrary|LogInfo (Utilities|String|ToString(Text) (Utilities|Text|FormatText "Stopped stream {id} ({type}): {reason}" StreamId (Utilities|TrackKind2String Kind) Reason))))

(event EventBeginPlay
  (bind _framesize (Variables|Default|GetframeSize))
  (bind (_x _y) (Utilities|Struct|BreakIntPoint _framesize))
  (|CallParentFunction)
  (Utilities|FlowControl|Sequence
    (:then_0
      (CallFunction|SetupRenderTarget _x _y)
      (CallFunction|SetupRTCMediaSender))
    (:then_1
      (Class|VideoCoreMediaSender|Init (Variables|Default|GetrtcSender) (CallFunction|GetVideoCoreSignalingComponent)))
    (:then_2
      (CallFunction|SetupCallbacks))))

(event Collision|EventActorBeginOverlap
  (params (OtherActor :type Actor%20Object%20Reference))
  (|CallParentFunction OtherActor) ; This node is disabled and will not be called.\nDrag off pins to build functionality.
)

(event EventTick
  (params (DeltaSeconds :type Float%20%28single-precision%29))
  (|CallParentFunction DeltaSeconds) ; This node is disabled and will not be called.\nDrag off pins to build functionality.
)

(fn ConstructionScript
  (|CallParentFunction))

(fn SetupRenderTarget
  (params (width :type Integer) (height :type Integer))
  (Utilities|IsValid (Variables|Default|GettextureRenderTarget)
    (:Is%20Valid
      _)
    (:Is%20Not%20Valid
      (bind _returnvalue (Rendering|CreateRenderTarget2D width height "RTF_RGBA8_SRGB"))
      (Variables|Default|SettextureRenderTarget _returnvalue)))
  (Variables|/Script/Engine.SceneCaptureComponent2D|SetTextureTarget (Variables|Default|GetSceneCaptureComponent2D) (Variables|Default|GettextureRenderTarget))
  (Rendering|Material|SetTextureParameterValue (Variables|Default|GetmyMaterialInstance) "Video Texture" (Variables|Default|GettextureRenderTarget))
  (Rendering|Material|SetScalarParameterValue (Variables|Default|GetmyMaterialInstance) "Enable Video Texture" 1.0 :!class /Script/Engine.MaterialInstanceDynamic)
  (CallFunction|UpdateKeyingParameters))

(fn SetupRTCMediaSender
  (bind _streamhint (Variables|Default|GetstreamHint))
  (bind _returnvalue (Game|ConstructObjectfromClass "/Script/VideoCoreRTC.VideoCoreMediaSender" self))
  (Variables|Default|SetrtcSender _returnvalue)
  (Variables|/Script/VideoCoreRTC.VideoCoreMediaSender|SetFrameRate (Variables|Default|GetrtcSender) (Variables|Default|Getfps))
  (Variables|/Script/VideoCoreRTC.VideoCoreMediaSender|SetFrameSize (Variables|Default|GetrtcSender) (Variables|Default|GetframeSize))
  (Variables|/Script/VideoCoreRTC.VideoCoreMediaSender|SetRenderTarget (Variables|Default|GetrtcSender) (Variables|Default|GettextureRenderTarget))
  (Variables|/Script/VideoCoreRTC.VideoCoreMediaSender|SetAutoProduce (Variables|Default|GetrtcSender) (Variables|Default|GetautoProduce))
  (Variables|/Script/VideoCoreRTC.VideoCoreMediaSender|SetBitrates (Variables|Default|GetrtcSender) (Variables|Default|Getbitrates))
  (Variables|/Script/VideoCoreRTC.VideoCoreMediaSender|SetVideoStreamHint (Variables|Default|GetrtcSender) _streamhint)
  (Variables|/Script/VideoCoreRTC.VideoCoreMediaSender|SetAudioStreamHint (Variables|Default|GetrtcSender) _streamhint))

(fn DrawHelperAxes
  ;[1 1 1] do nothing
)

(fn SetIsGrabbed
  (params (isGrabbed :type Boolean))
  (|CallParentFunction isGrabbed)
  (Development|SetHiddeninGame (Variables|Default|GetgrabSphere) true true))