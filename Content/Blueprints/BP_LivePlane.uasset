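; Webcam plane pawn that shows a live camera feed on its surface, built on a parent plane class.
; BeginPlay enables player input, sets floating movement speed and constrains movement on the Z axis.
; Tick runs the base plane update and pushes the webcam texture into the dynamic material; SetDeviceId switches webcams only when the ID changes.
; The V key alternates third- and first-person cameras, toggling controller-driven rotation.
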(event EventBeginPlay
  ;[0.02416 0.7379 1] Set up
  (|CallParentFunction)
  (Utilities|FlowControl|Sequence
    (:then_0
      (Input|EnableInput (Game|GetPlayerController 0))
      (Variables|Default|SetdefaultScale (Variables|/Script/Engine.SceneComponent|GetRelativeScale3D (Variables|Default|GetPlane)))
      (Variables|/Script/Engine.FloatingPawnMovement|SetMaxSpeed (Actor|GetComponentbyClass self "/Script/Engine.FloatingPawnMovement") 6e+02)
      (CallFunction|InitializeCameraPlane))
    (:then_1
      (Class|MovementComponent|SetPlaneConstraintAxisSetting (Variables|Default|GetMovementComponent) "Z"))))

(event EventTick
  (params (DeltaSeconds :type Float%20%28single-precision%29))
  ;[1 0 0] TICK
  (Utilities|FlowControl|Sequence
    (:then_0
      (CallFunction|PlaneBaseTick))
    (:then_1
      ;;[1 1 1] Webcam texture update
      (bind _returnvalue (Class|WebCameraComponent|GetTexture (Variables|Default|GetWebCamera)))
      (Rendering|Material|SetTextureParameterValue (Variables|Default|GetmyMaterialInstance) "Texture" _returnvalue))))

(event Input|KeyboardEvents|V
  (params (Key :type Key%20Structure))
  (bind _fp_camera (Variables|Default|GetFP_Camera))
  ;[1 0.677 0.07432] 1st/3rd person camera switch
  (:Pressed
    (Utilities|FlowControl|MultiGate false true -1
      (:Out%200
        (Variables|/Script/Engine.SpringArmComponent|SetTargetArmLength (Variables|Default|GetSpringArm_0) 3e+02)
        (Components|Activation|SetActive (Variables|Default|GetFP_Camera) false false)
        (Components|Activation|SetActive (Variables|Default|GetTP_Camera_0) true false)
        (Variables|Default|SetbUseControllerRotationPitch false)
        (Variables|Default|SetbUseControllerRotationRoll false)
        (Variables|Default|SetbUseControllerRotationYaw false))
      (:Out%201
        (Components|Activation|SetActive _fp_camera true false)
        (Components|Activation|SetActive (Variables|Default|GetTP_Camera_0) false true)
        (Transformation|SetRelativeLocation _fp_camera "0, 0, 0" false false)
        (Variables|Default|SetbUseControllerRotationPitch true)
        (Variables|Default|SetbUseControllerRotationRoll true)
        (Variables|Default|SetbUseControllerRotationYaw true)))))

(fn ConstructionScript
  (|CallParentFunction))

(fn InitializeCameraPlane
  (CallFunction|ResetFrameSelection)
  (CallFunction|SetDeviceId (Variables|Default|GetdeviceID))
  (return))

(fn SetDeviceId
  (params (deviceId :type Integer))
  (if (not (== deviceId (Variables|Default|GetdeviceID)))
    (bind _output_get (Variables|Default|SetdeviceID deviceId))
    (if (>= _output_get 0)
      (Class|WebCameraComponent|SetDeviceId (Variables|Default|GetWebCamera) _output_get)
      (CallFunction|ResetCameraTexture)
      (Class|DDBlueprintLibrary|LogDebug (Utilities|String|ToString(Text) (Utilities|Text|FormatText "set device {id}" _output_get))))))

(fn GetDeviceId
  (return (Variables|Default|GetdeviceID)))

(fn ResetCameraTexture
  (bind _returnvalue (Class|WebCameraComponent|GetTexture (Variables|Default|GetWebCamera)))
  (Rendering|Material|SetTextureParameterValue (Variables|Default|GetmyMaterialInstance) "Video Texture" _returnvalue)
  (Class|DDBlueprintLibrary|LogInfo "RESET CAMERA TEXTURE"))

(fn GetPlaneDebugString3
  (return (Utilities|String|ToString(Text) (Utilities|Text|FormatText "{str} 
device idx: {didx}" (|CallParentFunction) (Variables|Default|GetdeviceID)))))

(fn PostDeserializeInit
  (|CallParentFunction))