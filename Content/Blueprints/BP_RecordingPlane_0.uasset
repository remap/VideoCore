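; BP_RecordingPlane_0 is an actor Blueprint with an unfinished toggle for recording render target frames to disk.
; The Y key drives a FlipFlop that alternately sets and clears the Record flag, printing a message when recording starts.
; A Record-gated render target export to a hardcoded desktop path and fixed filename is disconnected, so nothing is saved.
; An unused Append hints at frame-numbered output; BeginPlay and Tick only call the parent.
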(event EventBeginPlay
  (|CallParentFunction))

(event Collision|EventActorBeginOverlap
  (params (OtherActor :type Actor%20Object%20Reference)))

(event EventTick
  (params (DeltaSeconds :type Float%20%28single-precision%29))
  (|CallParentFunction DeltaSeconds))

(event Input|KeyboardEvents|Y
  (params (Key :type Key%20Structure))
  (:Pressed
    (Utilities|FlowControl|FlipFlop
      (:A
        (Variables|Default|SetbRecord true)
        (Development|PrintString "record"))
      (:B
        (Variables|Default|SetbRecord false)))))

(fn ConstructionScript
  (|CallParentFunction))