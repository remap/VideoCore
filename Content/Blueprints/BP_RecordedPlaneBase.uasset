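; Base Blueprint for a recorded video plane that turns to match the camera of a pawn assigned through SetFacePawn.
; Tick copies that pawn's camera rotation to the root each frame, without the 180-degree flip used by PlaneParent, so the video stays visible.
; RotateToCamera stores a transform in PawnTransform, whose OnRep applies it to the actor only when no valid pawn is set to look at.
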(event Custom|RotateToCamera
  (params (NewTransform :type Transform))
  (Variables|Default|SetpawnTransform NewTransform))

(event EventBeginPlay)

(event Collision|EventActorBeginOverlap
  (params (OtherActor :type Actor%20Object%20Reference)))

(event EventTick
  (params (DeltaSeconds :type Float%20%28single-precision%29))
  (bind _self self)
  (bind _pawntolookat (Variables|Default|GetPawnToLookAt))
  (bind _rootcomponent (Variables|Transformation|GetRootComponent _self))
  (Utilities|FlowControl|Sequence
    (:then_0
      (if (Utilities|IsValid _pawntolookat)
        (Transformation|SetWorldRotation _rootcomponent (Transformation|GetWorldRotation (Actor|GetComponentbyClass _pawntolookat "/Script/Engine.CameraComponent")) false false)
        ;[1 1 1] unlike PlaneParent we don't rotate 180 here because if we do, the video will be facing outwards and we won't see th render
        (Transformation|AddLocalRotation _rootcomponent "0,0.000000, 0" false false)))
    (:then_1)))

(fn ConstructionScript)

(fn OnRepPawnTransform
  (if (not (Utilities|IsValid (Variables|Default|GetPawnToLookAt)))
    (Transformation|SetActorTransform (Variables|Default|GetpawnTransform))))

(fn SetFacePawn
  (params (pawn :type Pawn%20Object%20Reference))
  (bind _output_get (Variables|Default|SetPawnToLookAt pawn))
  (if (Utilities|IsValid _output_get)
    _))