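; Broadcaster actor that streams a scene capture as live video over RTC using VideoCore.
; On BeginPlay it creates a render target if none exists, assigns it to the SceneCapture2D and shows it on a material instance with updated keying parameters.
; It then builds a VideoCore media sender from that target, frame size and FPS, initializes it with the signaling component and starts producing a video track.
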(event EventBeginPlay
  (bind _framesize (Variables|Default|GetframeSize))
  (bind (_x _y) (Utilities|Struct|BreakIntPoint _framesize))
  (|CallParentFunction)
  (Utilities|FlowControl|Sequence
    (:then_0
      (CallFunction|CreateRenderTarget _x _y)
      (CallFunction|CreateRTCMediaSender))
    (:then_1
      (bind _returnvalue (Class|VideoCoreMediaSender|Produce (Variables|Default|GetrtcSender) "" "Video"))
      (Class|DDBlueprintLibrary|LogTrace (Utilities|String|ToString(Text) (Utilities|Text|FormatText "Start Producing video: {b}" _returnvalue))))))

(event Collision|EventActorBeginOverlap
  (params (OtherActor :type Actor%20Object%20Reference))
  (|CallParentFunction OtherActor) ; This node is disabled and will not be called.\nDrag off pins to build functionality.
)

(event EventTick
  (params (DeltaSeconds :type Float%20%28single-precision%29))
  (|CallParentFunction DeltaSeconds) ; This node is disabled and will not be called.\nDrag off pins to build functionality.
)

(fn ConstructionScript
  (|CallParentFunction))

(fn CreateRenderTarget
  (params (width :type Integer) (height :type Integer))
  (Utilities|IsValid (Variables|Default|GettextureRenderTarget)
    (:Is%20Valid
      _)
    (:Is%20Not%20Valid
      (bind _returnvalue (Rendering|CreateRenderTarget2D width height "RTF_RGBA8_SRGB"))
      (Variables|Default|SettextureRenderTarget _returnvalue)))
  (Variables|/Script/Engine.SceneCaptureComponent2D|SetTextureTarget (Variables|Default|GetSceneCaptureComponent2D) (Variables|Default|GettextureRenderTarget))
  (Rendering|Material|SetTextureParameterValue (Variables|Default|GetmyMaterialInstance) "Video Texture" (Variables|Default|GettextureRenderTarget))
  (Rendering|Material|SetScalarParameterValue (Variables|Default|GetmyMaterialInstance) "Enable Video Texture" 1.0 :!class /Script/Engine.MaterialInstanceDynamic)
  (CallFunction|UpdateKeyingParameters))

(fn CreateRTCMediaSender
  (bind _returnvalue (Game|ConstructObjectfromClass "/Script/VideoCoreRTC.VideoCoreMediaSender" self))
  (Variables|Default|SetrtcSender _returnvalue)
  (Variables|/Script/VideoCoreRTC.VideoCoreMediaSender|SetFrameRate (Variables|Default|GetrtcSender) (Variables|Default|Getfps))
  (Variables|/Script/VideoCoreRTC.VideoCoreMediaSender|SetFrameSize (Variables|Default|GetrtcSender) (Variables|Default|GetframeSize))
  (Variables|/Script/VideoCoreRTC.VideoCoreMediaSender|SetRenderTarget (Variables|Default|GetrtcSender) (Variables|Default|GettextureRenderTarget))
  (Class|VideoCoreMediaSender|Init (Variables|Default|GetrtcSender) (CallFunction|GetVideoCoreSignalingComponent)))