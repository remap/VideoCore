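; NDI video plane that re-streams its NDI source over RTC, acting as sender or receiver according to its RtcSenderReceiver role.
; First Tick claims ownership through the server to become sender; with RenderServerOnly, non-render-server instances instead show the received stream on their material.
; Senders create a render target when streaming starts, produce RTC video from it and copy the video texture into it each Tick via canvas drawing.
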(event Custom|On%20Consuming%20Started
  (params (ProducerId :type String) (Kind :type EMediaTrackKind%20Enum :default "Unknown"))
  (CallFunction|SetVideoTextureEnabled true))

(event Custom|On%20Consuming%20Stopped
  (params (ProducerId :type String) (Kind :type EMediaTrackKind%20Enum :default "Unknown") (Reason :type String))
  (CallFunction|SetVideoTextureEnabled false))

(event EventBeginPlay
  (|CallParentFunction) ; This node is disabled and will not be called.\nDrag off pins to build functionality.
)

(event Collision|EventActorBeginOverlap
  (params (OtherActor :type Actor%20Object%20Reference))
  (|CallParentFunction OtherActor) ; This node is disabled and will not be called.\nDrag off pins to build functionality.
)

(event EventTick
  (params (DeltaSeconds :type Float%20%28single-precision%29))
  (bind _helper (CallFunction|GetPlayerControllerHelper))
  (bind _self self)
  (bind _rtcsenderreceiver (Variables|Default|GetRtcSenderReceiver))
  (bind _playercontroller (Default|GetOwnerPlayerController _helper))
  (bind _mediareceiver (Variables|/VideoCore/Blueprints/BP_RtcSenderReceiverComponent.BP_RtcSenderReceiverComponent_C|GetmediaReceiver _rtcsenderreceiver))
  (|CallParentFunction DeltaSeconds)
  (Utilities|FlowControl|Sequence
    (:then_0
      (if (not (Variables|Default|GetisInitialized))
        (Utilities|DEBUGROLEPRINT
          (:exec
            ;[1 0.2708 0.9165] check if Render Server instance. if so, this instance becomes RTC sender.
            ; to make it a sender, the owner of this actor must be our player controller
            ; to change the owner in mplayer, we must ask server to do it
            (if (Variables|RTC|GetrenderServerOnly)
              (if (Variables|/VideoCore/Blueprints/BP_VideoCorePlayerControllerHelper.BP_VideoCorePlayerControllerHelper_C|GetisRenderServerInstance _helper)
                (Actor|SetOwner _self _playercontroller :!label _label)
                (Default|ServerSetPlaneOwner (CallFunction|GetPlayerControllerHelper) _self _playercontroller)
                (else
                  (EventDispatchers|BindEventtoOnStreamingStarted _mediareceiver (EventDispatchers|CreateEvent :!event Custom|On%20Consuming%20Started))
                  (EventDispatchers|BindEventtoOnStreamingStopped _mediareceiver (EventDispatchers|CreateEvent :!event Custom|On%20Consuming%20Stopped))
                  ;;[1 0.7218 0] for non-RenderServer instances -- the only role is to receive RTC stream
                  (Rendering|Material|SetTextureParameterValue (Variables|Default|GetmyMaterialInstance) "Video Texture" (Default|GetLocalRenderTexture (Variables|Default|GetRtcSenderReceiver)))))
              (else
                (goto _label)))
            (bind _result (Default|Init (Variables|Default|GetRtcSenderReceiver) (CallFunction|GetVideoCoreSignalingComponent)))
            (if _result
              _
              (else
                (Class|DDBlueprintLibrary|LogError "NDI-RTC Plane: failed to initialize Rtc SenderReceiver")))
            (Variables|Default|SetisInitialized true)))
        (else
          (Utilities|FlowControl|Sequence
            (:then_0
              (if (not (Variables|Default|Getstopped))
                (Utilities|SwitchbyRole
                  (:Sender
                    (CallFunction|DrawRenderTarget)))))
            (:then_1)))))))

(fn ConstructionScript
  (|CallParentFunction))

(fn StartStreaming
  (bind _rtcsenderreceiver (Variables|Default|GetRtcSenderReceiver))
  (bind _rtcframesize (Variables|RTC|GetrtcFrameSize))
  (bind (_x _y) (Utilities|Struct|BreakIntPoint _rtcframesize))
  (Utilities|SwitchbyRole
    (:Sender
      (|CallParentFunction)
      ;[1 0 0.009895] setup RTC sender once -- after this, it'll broadcast whatever is in the texture target
      (Utilities|IsValid (Variables|RTC|GettextureRenderTarget)
        (:Is%20Not%20Valid
          (bind _returnvalue (Rendering|CreateRenderTarget2D _x _y "RTF_RGBA8_SRGB"))
          (Utilities|IsValid _returnvalue
            (:Is%20Valid
              (bind _output_get (Variables|RTC|SettextureRenderTarget _returnvalue))
              (Utilities|IsValid _rtcsenderreceiver
                (:Is%20Valid
                  (bind (_result _msg) (Default|StartProduce _rtcsenderreceiver "Video" _output_get (Variables|RTC|GetrtcFrameSize) (Variables|RTC|GetrtcBitrate) (Utilities|String|ToString(Text) (Utilities|Text|FormatText "NDI-{source}" (Variables|Default|GetndiSourceName)))))
                  (if (not _result)
                    (Class|DDBlueprintLibrary|LogError (Utilities|String|ToString(Text) (Utilities|Text|FormatText "NDI-RTC restream failed: {msg}" _msg)))))
                (:Is%20Not%20Valid
                  (Class|DDBlueprintLibrary|LogError "RTC Sender-Receiver is invalid"))))
            (:Is%20Not%20Valid
              (Class|DDBlueprintLibrary|LogError "NDI-RTC Plane: failed to create render target"))))))
    (:Receiver
      (Class|DDBlueprintLibrary|LogWarning (Utilities|String|ToString(Text) (Utilities|Text|FormatText "NDI-RTC plane: can not re-stream in non-sender role (current role {role})" (Utilities|Role2String))) :!label _label))
    (:Unowned
      (goto _label))))

(fn StopStreaming
  (params (showProxy :type Boolean))
  (Utilities|SwitchbyRole
    (:Sender
      (|CallParentFunction showProxy))))

(fn DrawRenderTarget
  (bind _texturerendertarget (Variables|RTC|GettextureRenderTarget))
  (Utilities|IsValid _texturerendertarget
    (:Is%20Valid
      (bind (_canvas _size _context) (Rendering|BeginDrawCanvastoRenderTarget _texturerendertarget))
      (Canvas|DrawTexture :self _canvas :RenderTexture (Variables|Default|GetvideoTexture) :ScreenSize _size :CoordinateSize "(X=1.000000,Y=1.000000)" :BlendMode "BLEND_Opaque" :PivotPoint "(X=0.500000,Y=0.500000)")
      (Rendering|EndDrawCanvastoRenderTarget _context))
    (:Is%20Not%20Valid
      (Class|DDBlueprintLibrary|LogWarning "NDI-RTC Plane: render target is not valid"))))

(fn OnRepVar
  (Class|DDBlueprintLibrary|LogError (Utilities|String|ToString(Text) (Utilities|Text|FormatText "*********** VARIABLE REPLICATED --- value {v}" false))))