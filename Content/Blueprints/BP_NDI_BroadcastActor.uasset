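; Actor that streams a scene capture view as an NDI video source.
; On BeginPlay it creates a render target for SceneCaptureComponent2D, wraps it in a runtime-constructed NDI media sender with configured size, frame rate and name, and initializes NDIBroadcast with it.
; It also spawns an NDIBroadcastActor bound to that sender, then optionally starts broadcasting.
; Start and stop functions control the stream, with initialization and start failures logged.
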(event EventBeginPlay
  (bind (_framewidth _frameheight _fps _sourcename) (Utilities|GetBroadcastParams))
  (Utilities|FlowControl|Sequence
    (:then_0
      (CallFunction|CreateRenderTarget _framewidth _frameheight)
      (CallFunction|InitNDISender _framewidth _frameheight _fps _sourcename)
      (CallFunction|SetupNDIBroadcastActor))
    (:then_1
      (if (Variables|Default|GetbroadcastOnBeginPlay)
        (CallFunction|StartBroadcast)))))

(event Collision|EventActorBeginOverlap
  (params (OtherActor :type Actor%20Object%20Reference)))

(event EventTick
  (params (DeltaSeconds :type Float%20%28single-precision%29)))

(fn ConstructionScript)

(fn CreateRenderTarget
  (params (width :type Integer) (height :type Integer))
  (bind _returnvalue (Rendering|CreateRenderTarget2D width height "RTF_RGBA8_SRGB"))
  (bind _output_get (Variables|Default|SettextureRenderTarget _returnvalue))
  (Variables|/Script/Engine.SceneCaptureComponent2D|SetTextureTarget (Variables|Default|GetSceneCaptureComponent2D) _output_get))

(fn InitNDISender
  (params (frameWidth :type Integer) (frameHeight :type Integer) (fps :type Integer) (SourceName :type String))
  (bind _returnvalue (Game|ConstructObjectfromClass "/Script/NDIIO.NDIMediaSender" self))
  (bind _output_get (Variables|Default|SetndiSender _returnvalue))
  (Variables|/Script/NDIIO.NDIMediaSender|SetRenderTarget _output_get (Variables|Default|GettextureRenderTarget))
  (Variables|/Script/NDIIO.NDIMediaSender|SetFrameSize _output_get (Utilities|Struct|MakeIntPoint frameWidth frameHeight))
  (Variables|/Script/NDIIO.NDIMediaSender|SetFrameRate _output_get (Class|KismetMathLibrary|MakeFrameRate fps 1))
  (Variables|/Script/NDIIO.NDIMediaSender|SetSourceName _output_get SourceName)
  (bind _returnvalue_2 (Class|NDIBroadcastComponent|InitializeSource (Variables|Default|GetNDIBroadcast) (Variables|Default|GetndiSender)))
  (if (not _returnvalue_2)
    (Class|DDBlueprintLibrary|LogError "INITIALIZE FAILED")))

(fn SetupNDIBroadcastActor
  (bind _returnvalue (Game|SpawnActorfromClass "/Script/NDIIO.NDIBroadcastActor" (Math|Transform|MakeTransform "0, 0, 0") "Undefined" self 0))
  (bind _output_get (Variables|Default|SetNDI%20Broadcast%20Actor _returnvalue))
  (Variables|/Script/NDIIO.NDIBroadcastActor|SetNDIMediaSource _output_get (Variables|Default|GetndiSender)))

(fn StartBroadcast
  (bind (_errormessage _returnvalue) (Class|NDIBroadcastComponent|StartBroadcasting (Variables|Default|GetNDIBroadcast)))
  (if (not _returnvalue)
    (Class|DDBlueprintLibrary|LogError (Utilities|String|ToString(Text) (Utilities|Text|FormatText "Failed to start NDI broadcasting: {msg}" _errormessage)))))

(fn StopBroadcast
  (Class|NDIBroadcastComponent|StopBroadcasting (Variables|Default|GetNDIBroadcast)))