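; Video plane actor that displays an NDI stream on its mesh through an unlit chroma key material.
; Construction and BeginPlay link the video texture to an NDI media receiver (created if missing) and a dynamic material; only construction initializes the receiver component.
; Start/StopStreaming control that component for the selected source, toggling the material's video texture parameter.
; The debug string extends the parent's with connection and frame stats; receiver-actor spawning is unwired.
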(event EventBeginPlay
  (|CallParentFunction)
  (Utilities|FlowControl|Sequence
    (:then_0
      ;[1 1 1] ndi setup
      (NDI|SetupNDIVideoTexture)
      (NDI|SetupNDIReceiverSource)
      (NDI|SetupMaterialInstance))))

(event Collision|EventActorBeginOverlap
  (params (OtherActor :type Actor%20Object%20Reference))
  (|CallParentFunction OtherActor) ; This node is disabled and will not be called.\nDrag off pins to build functionality.
)

(event EventTick
  (params (DeltaSeconds :type Float%20%28single-precision%29))
  (|CallParentFunction DeltaSeconds) ; This node is disabled and will not be called.\nDrag off pins to build functionality.
)

(fn ConstructionScript
  (|CallParentFunction)
  (NDI|SetupNDIVideoTexture)
  (NDI|SetupNDIReceiverSource)
  (NDI|SetupMaterialInstance)
  (NDI|InitNDIReceiverComponent))

(fn SetNDISource
  (params (ndiSource :type NDI%20Connection%20Information%20Structure))
  (bind _output_get (Variables|NDI|SetndiSourceName (.SourceName (Utilities|Struct|BreakNDIConnectionInformation ndiSource))))
  (Variables|NDI|SetndiConnectionInfo ndiSource)
  (Class|DDBlueprintLibrary|LogTrace (Utilities|String|ToString(Text) (Utilities|Text|FormatText "set NDI source {n}" _output_get))))

(fn SetupNDIVideoTexture
  (Utilities|IsValid (Variables|NDI|GetvideoTexture)
    (:Is%20Valid
      (Class|DDBlueprintLibrary|LogInfo "Video texture is setup using Blueprints"))
    (:Is%20Not%20Valid
      (Class|DDBlueprintLibrary|LogInfo "Create NDI video texture"))))

(fn SetupNDIReceiverSource
  (Utilities|IsValid (Variables|NDI|GetreceiverSource)
    (:Is%20Valid
      (Class|DDBlueprintLibrary|LogInfo "NDI Source is set in Blueprint defaults"))
    (:Is%20Not%20Valid
      (Class|DDBlueprintLibrary|LogInfo "Creating receiver NDI source")
      (bind _returnvalue (Game|ConstructObjectfromClass "/Script/NDIIO.NDIMediaReceiver" self))
      (bind _output_get (Variables|NDI|SetreceiverSource _returnvalue))))
  (Utilities|IsValid (Variables|/Script/NDIIO.NDIMediaReceiver|GetVideoTexture _output_get)
    (:Is%20Valid
      _)
    (:Is%20Not%20Valid
      _))
  (Variables|/Script/NDIIO.NDIMediaReceiver|SetVideoTexture _output_get (Variables|NDI|GetvideoTexture))
  (Class|DDBlueprintLibrary|LogTrace "SET VIDEO TEXTURE")
  (Utilities|IsValid (Variables|NDI|GetreceiverSource)
    (:Is%20Not%20Valid
      (Class|DDBlueprintLibrary|LogError "NDI plane: Could not setup NDI receiver source"))))

(fn SetupMaterialInstance
  (Utilities|IsValid (Variables|NDI|GetmaterialInstance)
    (:Is%20Valid
      (Class|DDBlueprintLibrary|LogInfo "NDI material instance is setup in Blueprints"))
    (:Is%20Not%20Valid
      (Class|DDBlueprintLibrary|LogInfo "Creating NDI material instance")))
  (bind _returnvalue (Rendering|Material|CreateDynamicMaterialInstance (Variables|Default|GetPlane) 0 "/VideoCore/Materials/M_VideoCore_NDI_Unlit_ChromaKey.M_VideoCore_NDI_Unlit_ChromaKey" "MI_NDI_Chroma" :!class /Script/Engine.PrimitiveComponent))
  (bind _output_get (Variables|NDI|SetmaterialInstance _returnvalue))
  (Rendering|Material|SetTextureParameterValue _output_get "Video Texture" (Variables|NDI|GetvideoTexture))
  (Rendering|Material|SetTextureParameterValue (Variables|NDI|GetmaterialInstance) "Proxy Texture" (Variables|NDI|GetproxyTexture)))

(fn StartStreaming
  (CallFunction|StopStreaming)
  (bind _returnvalue (Class|NDIReceiverComponent|StartReceiver (Variables|Default|GetNDIReceiver) (Variables|NDI|GetndiConnectionInfo)))
  (NDI|SetVideoTextureEnabled _returnvalue)
  (Class|DDBlueprintLibrary|LogInfo (select _returnvalue "Started NDI receiver" "Failed to start NDI receiver")))

(fn StopStreaming
  (Class|NDIReceiverComponent|ShutdownReceiver (Variables|Default|GetNDIReceiver))
  (NDI|SetVideoTextureEnabled false))

(fn SetupNDIReceiverActor
  (Class|DDBlueprintLibrary|LogInfo "Spawning NDI Receive Actor")
  (bind _returnvalue (Game|SpawnActorfromClass "/Script/NDIIO.NDIReceiveActor" (Transformation|GetActorTransform self) "Undefined" self 0))
  (Transformation|AddActorLocalRotation _returnvalue "180.000000,0.000000, 0" false false)
  (Utilities|IsValid _returnvalue
    (:Is%20Valid
      (bind _output_get (Variables|NDI|SetreceiveActor _returnvalue))
      (Variables|/Script/NDIIO.NDIReceiveActor|SetNDIMediaSource _output_get (Variables|NDI|GetreceiverSource))
      (Class|NDIReceiveActor|SetupMediaSource _output_get))
    (:Is%20Not%20Valid
      (Class|DDBlueprintLibrary|LogError "Failed to spawn NDI receive actor"))))

(fn InitNDIReceiverComponent
  (bind _returnvalue (Class|NDIReceiverComponent|Initialize (Variables|Default|GetNDIReceiver) (Variables|NDI|GetreceiverSource)))
  (if (not _returnvalue)
    (Class|DDBlueprintLibrary|LogError "Failed initialize receiver component")))

(fn SetVideoTextureEnabled
  (params (enabled :type Boolean))
  (Rendering|Material|SetScalarParameterValue (Variables|NDI|GetmaterialInstance) "Enable Video Texture" (select enabled 1.0 0.0) :!class /Script/Engine.MaterialInstanceDynamic))

(fn GetPlaneDebugString
  (bind _receiversource (Variables|NDI|GetreceiverSource))
  (bind _performancedata (Variables|/Script/NDIIO.NDIMediaReceiver|GetPerformanceData _receiversource))
  (bind _connectioninformation (Variables|/Script/NDIIO.NDIMediaReceiver|GetConnectionInformation _receiversource))
  (bind (_audioframes _droppedvideoframes _droppedaudioframes _droppedmetadataframes _metadataframes _videoframes) (Utilities|Struct|BreakNDIReceiverPerformanceData _performancedata))
  (bind (_sourcename _machinename _streamname _url _bandwidth _biscurrentlyconnected) (Utilities|Struct|BreakNDIConnectionInformation _connectioninformation))
  (return (Utilities|String|ToString(Text) (Utilities|Text|FormatText "{p} 
source: {ndiSource} 
connected: {c} 
source URL: {url} 
b/w: {bw} 
a frames: {a}/{da} 
v frames: {v}/{dv} 
m frames: {m}/{dm}" (|CallParentFunction) (Variables|NDI|GetndiSourceName) _biscurrentlyconnected _url (Utilities|Select :Index _bandwidth :MetadataOnly "metadata" :AudioOnly "audio" :Lowest "lowest" :Highest "highest") (Math|Conversions|ToInteger(Byte) _audioframes) (Math|Conversions|ToInteger(Byte) _droppedaudioframes) (Math|Conversions|ToInteger(Byte) _videoframes) (Math|Conversions|ToInteger(Byte) _droppedvideoframes) (Math|Conversions|ToInteger(Byte) _metadataframes) (Math|Conversions|ToInteger(Byte) _droppedmetadataframes)))))