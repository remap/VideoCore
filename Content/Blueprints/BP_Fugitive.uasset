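; BP_Fugitive is the fugitive actor Blueprint, extending a parent that supplies its begin-play and tick behavior.
; After a half-second delay on BeginPlay, it runs the parent logic, initializes a camera plane, stores the returned material instance and sets Pause.
; While Pause is true, each Tick passes that material, marked deprecated, to GlobalTick.
; A RepNotify applies a replicated transform to the actor; the material's RepNotify is empty.
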(event EventBeginPlay
  (Utilities|FlowControl|Delay 0.5)
  (|CallParentFunction)
  (bind _thematerialinstance (CallFunction|InitializeCameraPlane))
  (Variables|Default|SetmyMaterialInstance_DEPRECATED _thematerialinstance)
  (Variables|Default|SetPause true))

(event EventTick
  (params (DeltaSeconds :type Float%20%28single-precision%29))
  (|CallParentFunction DeltaSeconds)
  (if (Variables|Default|GetPause)
    (CallFunction|GlobalTick (Variables|Default|GetmyMaterialInstance_DEPRECATED))))

(fn ConstructionScript
  (|CallParentFunction))

(fn OnRepPawnTransform0
  (Transformation|SetActorTransform (Variables|Default|GetpawnTransform_0)))

(fn OnRepMyMaterialInstance)