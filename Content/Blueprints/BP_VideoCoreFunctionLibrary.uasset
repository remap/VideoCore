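; Blueprint function library for the video core, giving shared lookups for camera plane actors and the player controller helper.
; Plane getters gather all, live or recorded planes by class, though the live getter still uses the parent plane class as a marked placeholder.
; A name search loops over all planes comparing PawnName and reports whether one is found.
; The helper getter fetches the VideoCore helper component from the first player controller.
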(fn GetAllPlanes
  (bind _outactors (Actor|GetAllActorsOfClass 0 "/VideoCore/Blueprints/BP_CameraPlaneParent.BP_CameraPlaneParent_C"))
  (return _outactors))

(fn GetLivePlanesOnly
  ;[1 0 0.2503] THIS MUST BE REPLACED WITH LIVE PLANE CLASS
  (bind _outactors (Actor|GetAllActorsOfClass 0 "/VideoCore/Blueprints/BP_CameraPlaneParent.BP_CameraPlaneParent_C"))
  (return _outactors))

(fn GetRecordedPlanesOnly
  (bind _outactors (Actor|GetAllActorsOfClass 0 "/VideoCore/Blueprints/BP_RecordedPlaneBase.BP_RecordedPlaneBase_C"))
  (return _outactors))

(fn GetPlayerControllerHelper
  (return (Actor|GetComponentbyClass (Game|GetPlayerController 0) "/VideoCore/Blueprints/BP_VideoCorePlayerControllerHelper.BP_VideoCorePlayerControllerHelper_C")))

(fn FindPlanebyName
  (params (planeName :type String))
  (for _array_element (CallFunction|GetAllPlanes)
    (if (Utilities|Enum|Equal(Enum) (Variables|/VideoCore/Blueprints/BP_CameraPlaneParent.BP_CameraPlaneParent_C|GetpawnName _array_element) (Utilities|Text|ToText(String) planeName))
      (return _array_element true)))
  (return 0 false))